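; BP_Generate sets up the round's medical case at BeginPlay, using a fixed tutorial diagnosis or a random one.
; The construction script fills the random pool from the Asset Registry with diagnosis data assets.
; The chosen diagnosis's information and symptoms feed the InfoDiag and Memory lists, and BP_Validation receives it as the answer.
; Each BP_Machine gets type-matched diagnosis info and is lit, otherwise taking default output from InfoBase.
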(event EventBeginPlay
  (bind _all_diagnostique (Variables|Default|Getall_diagnostique))
  (if (Variables|Default|Gettuto)
    (Variables|Default|Setdiagnostique_to_do "/Game/Data_Asset/Diagnostique/Membre_Platre/DA_Diag_Jambe_Droite_Platre.DA_Diag_Jambe_Droite_Platre")
    (else
      (Variables|Default|Setdiagnostique_to_do (Utilities|Array|Get(acopy) _all_diagnostique (- (Math|Random|RandomIntegerinRange 1 (Utilities|Array|Length _all_diagnostique)) 1)))))
  (for _array_element (Variables|/Game/Blueprint/Primary_Data_Asset/BP_PDA_Diagnostique.BP_PDA_Diagnostique_C|Getlist_information (Variables|Default|Getdiagnostique_to_do))
    (if (Utilities|Enum|Equal(Enum) (Variables|/Game/Blueprint/Primary_Data_Asset/BP_PDA_Item.BP_PDA_Item_C|Getmemory _array_element) "NewEnumerator1")
      (Utilities|Array|Add (Variables|Default|Getmemory) _array_element))
    (Utilities|Array|Add (Variables|Default|Getinfo_diag) _array_element))
  (for _array_element_2 (Variables|/Game/Blueprint/Primary_Data_Asset/BP_PDA_Diagnostique.BP_PDA_Diagnostique_C|Getlist_symptome (Variables|Default|Getdiagnostique_to_do))
    (if (Utilities|Enum|Equal(Enum) (Variables|/Game/Blueprint/Primary_Data_Asset/BP_PDA_Item.BP_PDA_Item_C|Getmemory _array_element_2) "NewEnumerator1")
      (Utilities|Array|Add (Variables|Default|Getmemory) _array_element_2))
    (for _array_element_3 (Variables|/Game/Blueprint/Primary_Data_Asset/BP_PDA_Symptome.BP_PDA_Symptome_C|Getlist_information _array_element_2)
      (if (Utilities|Enum|Equal(Enum) (Variables|/Game/Blueprint/Primary_Data_Asset/BP_PDA_Item.BP_PDA_Item_C|Getmemory _array_element_3) "NewEnumerator1")
        (Utilities|Array|Add (Variables|Default|Getmemory) _array_element_3))
      (Utilities|Array|Add (Variables|Default|Getinfo_diag) _array_element_3)))
  (bind _returnvalue (Actor|GetActorOfClass "/Game/Blueprint/Machines/BP_Validation.BP_Validation_C"))
  (Variables|/Game/Blueprint/Machines/BP_Validation.BP_Validation_C|Setvalidation _returnvalue (Variables|Default|Getdiagnostique_to_do))
  (bind _outactors (Actor|GetAllActorsOfClass "/Game/Blueprint/Machines/BP_Machine.BP_Machine_C"))
  (for _array_element_4 _outactors
    (for _array_element_5 (Variables|Default|Getinfo_diag)
      (if (Utilities|Enum|Equal(Enum) (Variables|/Game/Blueprint/Primary_Data_Asset/BP_PDA_Item.BP_PDA_Item_C|Gettype _array_element_5) (Variables|/Game/Blueprint/Machines/BP_Machine.BP_Machine_C|Gettype _array_element_4))
        (Variables|/Game/Blueprint/Machines/BP_Machine.BP_Machine_C|Setitem_out _array_element_4 _array_element_5)
        (Variables|/Game/Blueprint/Machines/BP_Machine.BP_Machine_C|Setdo_it _array_element_4 true)
        (Default|SetLight _array_element_4)))
    (if (not (Variables|/Game/Blueprint/Machines/BP_Machine.BP_Machine_C|Getdo_it _array_element_4))
      (for _array_element_6 (Variables|Default|Getinfo_base)
        (if (Utilities|Enum|Equal(Enum) (Variables|/Game/Blueprint/Primary_Data_Asset/BP_PDA_Item.BP_PDA_Item_C|Gettype _array_element_6) (Variables|/Game/Blueprint/Machines/BP_Machine.BP_Machine_C|Gettype _array_element_4))
          (Variables|/Game/Blueprint/Machines/BP_Machine.BP_Machine_C|Setitem_out _array_element_4 _array_element_6))))))

(fn ConstructionScript
  (bind _outassetdata (Class|AssetRegistry|GetAssetsbyClass (Class|AssetRegistryHelpers|GetAssetRegistry) (Class|KismetSystemLibrary|GetClassTopLevelAssetPath "/Game/Blueprint/Primary_Data_Asset/BP_PDA_Diagnostique.BP_PDA_Diagnostique_C") false))
  (for _array_element _outassetdata
    (bind _asbp_pda_diagnostique (Utilities|Casting|CastToBP_PDA_Diagnostique (Class|AssetRegistryHelpers|GetAsset _array_element)))
    (Utilities|Array|Add (Variables|Default|Getall_diagnostique) _asbp_pda_diagnostique)))