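; BP_Item is a world pickup that displays an item asset and moves it into the first-person player controller's inventory on interaction.
; Interract writes the item into the selected slot, destroying the actor if the slot held DA_Item_Void, otherwise taking on the displaced item as a swap.
; Charge, run at BeginPlay and after swaps, applies the item's mesh and hard-codes a matching material for each of four Disquette meshes.
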(event EventBeginPlay
  (|CallParentFunction)
  (Variables|Default|Setglowing true)
  (Utilities|IsValid (Variables|Default|Getitem)
    (:Is%20Valid
      (CallFunction|Charge))))

(event Collision|EventActorBeginOverlap
  (params (OtherActor :type Actor%20Object%20Reference))
  (|CallParentFunction OtherActor) ; This node is disabled and will not be called.\nDrag off pins to build functionality.
)

(event EventTick
  (params (DeltaSeconds :type Float%20%28single-precision%29))
  (|CallParentFunction DeltaSeconds) ; This node is disabled and will not be called.\nDrag off pins to build functionality.
)

(fn ConstructionScript
  (|CallParentFunction))

(fn Interract
  (|CallParentFunction)
  (bind _asbp_first_person_player_controller (Utilities|Casting|CastToBP_FirstPersonPlayerController (Game|GetPlayerController 0)))
  (if (== (Utilities|Array|Get(acopy) (Variables|/Game/FirstPerson/Blueprints/BP_FirstPersonPlayerController.BP_FirstPersonPlayerController_C|Getinventory _asbp_first_person_player_controller) (Variables|/Game/FirstPerson/Blueprints/BP_FirstPersonPlayerController.BP_FirstPersonPlayerController_C|Getselected_item _asbp_first_person_player_controller)) "/Game/Data_Asset/DA_Item_Void.DA_Item_Void")
    (Utilities|Array|Insert (Variables|/Game/FirstPerson/Blueprints/BP_FirstPersonPlayerController.BP_FirstPersonPlayerController_C|Getinventory _asbp_first_person_player_controller) (Variables|Default|Getitem) (Variables|/Game/FirstPerson/Blueprints/BP_FirstPersonPlayerController.BP_FirstPersonPlayerController_C|Getselected_item _asbp_first_person_player_controller))
    (Utilities|Array|RemoveIndex (Variables|/Game/FirstPerson/Blueprints/BP_FirstPersonPlayerController.BP_FirstPersonPlayerController_C|Getinventory _asbp_first_person_player_controller) (+ (Variables|/Game/FirstPerson/Blueprints/BP_FirstPersonPlayerController.BP_FirstPersonPlayerController_C|Getselected_item _asbp_first_person_player_controller) 1))
    (Actor|DestroyActor)
    (else
      (Utilities|Array|Insert (Variables|/Game/FirstPerson/Blueprints/BP_FirstPersonPlayerController.BP_FirstPersonPlayerController_C|Getinventory _asbp_first_person_player_controller) (Variables|Default|Getitem) (Variables|/Game/FirstPerson/Blueprints/BP_FirstPersonPlayerController.BP_FirstPersonPlayerController_C|Getselected_item _asbp_first_person_player_controller))
      (Variables|Default|Setitem (Utilities|Array|Get(acopy) (Variables|/Game/FirstPerson/Blueprints/BP_FirstPersonPlayerController.BP_FirstPersonPlayerController_C|Getinventory _asbp_first_person_player_controller) (+ (Variables|/Game/FirstPerson/Blueprints/BP_FirstPersonPlayerController.BP_FirstPersonPlayerController_C|Getselected_item _asbp_first_person_player_controller) 1)))
      (CallFunction|Charge)
      (Utilities|Array|RemoveIndex (Variables|/Game/FirstPerson/Blueprints/BP_FirstPersonPlayerController.BP_FirstPersonPlayerController_C|Getinventory _asbp_first_person_player_controller) (+ (Variables|/Game/FirstPerson/Blueprints/BP_FirstPersonPlayerController.BP_FirstPersonPlayerController_C|Getselected_item _asbp_first_person_player_controller) 1))))
  (for _array_element (Variables|/Game/FirstPerson/Blueprints/BP_FirstPersonPlayerController.BP_FirstPersonPlayerController_C|Getinventory _asbp_first_person_player_controller)
    _))

(fn Charge
  (bind _item (Variables|Default|Getitem))
  (bind _mesh (Variables|Character|GetMesh))
  (bind _mesh_2 (Variables|/Game/Blueprint/Primary_Data_Asset/BP_PDA_Item.BP_PDA_Item_C|Getmesh _item))
  (Components|StaticMesh|SetStaticMesh _mesh _mesh_2)
  (if (== _mesh_2 "/Game/Mesh/disquette_01.disquette_01")
    (Rendering|Material|SetMaterial _mesh 0 "/Game/Mesh/dis_01.dis_01")
    (elif (== _mesh_2 "/Game/Mesh/disquette_02.disquette_02")
      (Rendering|Material|SetMaterial _mesh 0 "/Game/Mesh/dis_02.dis_02")
      (elif (== _mesh_2 "/Game/Mesh/disquette_03.disquette_03")
        (Rendering|Material|SetMaterial _mesh 0 "/Game/Mesh/dis_03.dis_03")
        (elif (== _mesh_2 "/Game/Mesh/disquette_04.disquette_04")
          (Rendering|Material|SetMaterial _mesh 0 "/Game/Mesh/dis_04.dis_04"))))))