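; BP_Cable is an actor that draws a cable between two points, with the free end following the cursor until it is placed.
; On BeginPlay, DrawCable adds a cable component at StartPoint, ending at EndPoint, with length scaled down from their distance.
; While SecondPointSet is false, Tick moves the end to the under-cursor impact point.
; SetSecondPointPos only stores EndPoint; nothing here sets the flag or recomputes cable length.
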(event EventBeginPlay
  (CallFunction|DrawCable))

(event EventTick
  (params (DeltaSeconds :type Float%20%28single-precision%29))
  (if (not (Variables|Default|Getsecond_point_set))
    (CallFunction|SecondPointtoMouse)))

(fn ConstructionScript)

(fn DrawCable
  (bind _returnvalue (AddComponent|AddCableComponent false (Math|Transform|MakeTransform (Variables|Default|Getstart_point) "0, 0, 0" "1.000000,1.000000,1.000000")))
  (bind _output_get (Variables|Default|Setcable_comp _returnvalue))
  (Variables|/Script/CableComponent.CableComponent|SetEndLocation _output_get (Variables|Default|Getend_point))
  (Variables|/Script/CableComponent.CableComponent|SetCableLength (Variables|Default|Getcable_comp) (/ (Math|Vector|Distance(Vector) (Variables|Default|Getstart_point) (Variables|Default|Getend_point)) 2e+02))
  (Variables|/Script/CableComponent.CableComponent|SetCableWidth (Variables|Default|Getcable_comp) 0.5))

(fn SecondPointtoMouse
  (bind _impactpoint (CallFunction|GetUnderCursor))
  (bind _output_get (Variables|Default|Setend_point _impactpoint))
  (Variables|/Script/CableComponent.CableComponent|SetEndLocation (Variables|Default|Getcable_comp) _output_get))

(fn SetSecondPointPos
  (params (end_point :type Vector))
  (Variables|Default|Setend_point end_point))