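; Fusion machine where the player inserts held items as up to five discs, rotating the mesh with each insert, to craft diagnoses or symptoms.
; Items expand into information assets, which are matched by count and content against diagnoses first, then symptoms.
; A spawned button references the machine as parent.
; After a delayed spin, undiscovered results eject the inputs and any crafted item; the first success also triggers BP_Table's spawn.
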(event Custom|rotate
  (params (rotation_start :type Rotator))
  (bind _newtrack_0 (Timeline|Timeline PlayFromStart)
    (:Update
      (Transformation|SetWorldRotation (Variables|Character|GetMesh) (Math|Rotator|Lerp(Rotator) (Math|Rotator|MakeRotator 0.0 0.0 (.yaw rotation_start)) (Math|Rotator|MakeRotator 0.0 0.0 (+ (.yaw rotation_start) 72.0)) _newtrack_0) false false))))

(event Custom|rotateToZero
  (params (rotation_start :type Rotator) (rotation_added :type Float%20%28double-precision%29))
  (Components|Timeline|SetPlayRate (Variables|Default|GetTimeline_0) (/ 1.0 (/ rotation_added 72.0)))
  (bind _newtrack_0 (Timeline|Timeline_0 PlayFromStart)
    (:Update
      (Transformation|SetWorldRotation (Variables|Character|GetMesh) (Math|Rotator|Lerp(Rotator) (Math|Rotator|MakeRotator 0.0 0.0 (.yaw rotation_start)) (Math|Rotator|MakeRotator 0.0 0.0 (+ (.yaw rotation_start) rotation_added)) _newtrack_0) false false))))

(event Custom|createItem
  (params (time :type Float%20%28double-precision%29))
  (Utilities|FlowControl|Delay time)
  (Components|Animation|PlayAnimation (Variables|Default|GetEnigma) "/Game/Mesh/environement/Walls/Fusion_Wall/Animation/SK_fusion_wall_Anim.SK_fusion_wall_Anim" false)
  (bind _newtrack_0 (Timeline|Timeline_1 PlayFromStart)
    (:Update
      (Transformation|SetWorldRotation (Variables|Character|GetMesh) (Math|Rotator|Lerp(Rotator) "0, 0, 0" (Math|Rotator|MakeRotator 0.0 0.0 1.08e+03) _newtrack_0) false false))
    (:Finished
      (if (not (Utilities|Array|ContainsItem (Variables|/Game/FirstPerson/Blueprints/BP_FirstPersonPlayerController.BP_FirstPersonPlayerController_C|Getitem_find (CallFunction|GetController)) (Variables|Default|Getitem_to_out)))
        (for (_array_element _array_index) (Variables|Default|Getitem_fusion)
          (bind _returnvalue (Game|SpawnActorfromClass "/Game/Blueprint/BP_Item.BP_Item_C" (Math|Transform|MakeTransform (+ (Transformation|GetActorLocation) (Math|Vector|MakeVector 92.0 (- (Math|Conversions|ToFloat(Integer) (* _array_index 20)) 32.0) 73.0)) "0.000000,-90.000000,0.000000" "1.000000,1.000000,1.000000") "Undefined" "MultiplyWithRoot" 0 0))
          (Variables|/Game/Blueprint/BP_Item.BP_Item_C|Setitem _returnvalue _array_element)
          (Default|SetMesh _returnvalue)
          (switch int _array_index
            (:0
              (Rendering|SetVisibility (Variables|Default|Getdisc_01) false false))
            (:1
              (Rendering|SetVisibility (Variables|Default|Getdisc_02) false false))
            (:2
              (Rendering|SetVisibility (Variables|Default|Getdisc_03) false false))
            (:3
              (Rendering|SetVisibility (Variables|Default|Getdisc_04) false false))
            (:4
              (Rendering|SetVisibility (Variables|Default|Getdisc_05) false false))))
        (Utilities|IsValid (Variables|Default|Getitem_to_out)
          (:Is%20Valid
            (if (Variables|Default|Getfirst_fusion)
              (Variables|Default|Setfirst_fusion false)
              (bind _returnvalue_2 (Actor|GetActorOfClass "/Game/Blueprint/Machines/BP_Table.BP_Table_C"))
              (Default|Spawn _returnvalue_2))
            (bind _returnvalue_3 (Game|SpawnActorfromClass "/Game/Blueprint/BP_Item.BP_Item_C" (Math|Transform|MakeTransform (+ (Math|Vector|RotateVector (Variables|/Script/Engine.SceneComponent|GetRelativeLocation (Variables|Default|Getoutput)) (Transformation|GetActorRotation)) (Transformation|GetActorLocation)) "0.000000,-180.000000,-142.000000" "1.000000,1.000000,1.000000") "Undefined" "MultiplyWithRoot" 0 0))
            (Variables|/Game/Blueprint/BP_Item.BP_Item_C|Setitem _returnvalue_3 (Variables|Default|Getitem_to_out))
            (Default|SetMesh _returnvalue_3))
          (:Is%20Not%20Valid
            _))
        (Utilities|Array|Clear (Variables|Default|Getitem_fusion))))))

(event EventBeginPlay
  (bind _button_position (Variables|Default|Getbutton_position))
  (|CallParentFunction)
  (bind _returnvalue (Game|SpawnActorfromClass "/Game/Blueprint/Buttons/BP_Button_Fusion.BP_Button_Fusion_C" (Math|Transform|MakeTransform (+ (Transformation|GetActorLocation) (Variables|/Script/Engine.SceneComponent|GetRelativeLocation _button_position)) (Math|Rotator|CombineRotators (Transformation|GetActorRotation) (Variables|/Script/Engine.SceneComponent|GetRelativeRotation _button_position)) "1.000000,1.000000,1.000000") "Undefined" "MultiplyWithRoot" 0 0))
  (Variables|/Game/Blueprint/Buttons/BP_Button_Fusion.BP_Button_Fusion_C|Setmachine_parent _returnvalue self))

(event Collision|EventActorBeginOverlap
  (params (OtherActor :type Actor%20Object%20Reference))
  (|CallParentFunction OtherActor) ; This node is disabled and will not be called.\nDrag off pins to build functionality.
)

(event EventTick
  (params (DeltaSeconds :type Float%20%28single-precision%29))
  (|CallParentFunction DeltaSeconds) ; This node is disabled and will not be called.\nDrag off pins to build functionality.
)

(fn ConstructionScript
  (|CallParentFunction))

(fn Interract
  (bind _asbp_first_person_player_controller (CallFunction|GetController))
  (|CallParentFunction)
  (if (!= (Utilities|Array|Get(acopy) (Variables|/Game/FirstPerson/Blueprints/BP_FirstPersonPlayerController.BP_FirstPersonPlayerController_C|Getinventory _asbp_first_person_player_controller) (Variables|/Game/FirstPerson/Blueprints/BP_FirstPersonPlayerController.BP_FirstPersonPlayerController_C|Getselected_item _asbp_first_person_player_controller)) "/Game/Data_Asset/DA_Item_Void.DA_Item_Void")
    (CallFunction|AddItemFusion)
    (Default|SetIcons (Variables|/Game/FirstPerson/Blueprints/BP_FirstPersonPlayerController.BP_FirstPersonPlayerController_C|Getin_game_ui _asbp_first_person_player_controller))
    (CallFunction|Rotate (Transformation|GetWorldRotation (Variables|Character|GetMesh)))
    (else
      (Development|PrintString "main vide"))))

(fn CheckFusion
  (bind _item_check (Variables|Default|Getitem_check))
  (bind _item_check_2 (Variables|Default|Getitem_check))
  (bind _output (Utilities|Array|Get(acopy) _item_check_2))
  (bind _output_2 (Utilities|Array|Get(acopy) _item_check))
  (bind _list_diagnostique (Variables|/Game/Blueprint/Primary_Data_Asset/BP_PDA_Information.BP_PDA_Information_C|Getlist_diagnostique _output_2))
  (bind _list_symptome (Variables|/Game/Blueprint/Primary_Data_Asset/BP_PDA_Information.BP_PDA_Information_C|Getlist_symptome _output))
  (Variables|Default|Setitem_to_out 0)
  (bind (_array_element _array_index) (Utilities|Array|ForEachLoopwithBreak _list_diagnostique :!label _label)
    (:LoopBody
      (Variables|Default|Setset_item true)
      (Utilities|Array|Clear (Variables|Default|Getinfo_diag))
      (CallFunction|AddInfoDiag (Variables|/Game/Blueprint/Primary_Data_Asset/BP_PDA_Diagnostique.BP_PDA_Diagnostique_C|Getlist_information _array_element))
      (for _array_element_2 (Variables|/Game/Blueprint/Primary_Data_Asset/BP_PDA_Diagnostique.BP_PDA_Diagnostique_C|Getlist_symptome _array_element)
        (CallFunction|AddInfoDiag (Variables|/Game/Blueprint/Primary_Data_Asset/BP_PDA_Symptome.BP_PDA_Symptome_C|Getlist_information _array_element_2)))
      (if (== (Utilities|Array|Length (Variables|Default|Getitem_check)) (Utilities|Array|Length (Variables|Default|Getinfo_diag)))
        (CallFunction|CheckItemCheckContains (Variables|Default|Getinfo_diag))
        (if (Variables|Default|Getset_item)
          (if (Utilities|Enum|Equal(Enum) (Variables|/Game/Blueprint/Primary_Data_Asset/BP_PDA_Item.BP_PDA_Item_C|Getmemory (Utilities|Array|Get(acopy) _list_diagnostique _array_index)) "NewEnumerator0")
            (Variables|Default|Setitem_to_out (Utilities|Array|Get(acopy) _list_diagnostique _array_index))
            (goto _label Break)))))
    (:Completed
      (Utilities|IsValid (Variables|Default|Getitem_to_out)
        (:Is%20Valid
          (Development|PrintString "fusion diagnostique"))
        (:Is%20Not%20Valid
          (bind (_array_element_3 _array_index_2) (Utilities|Array|ForEachLoopwithBreak _list_symptome :!label _label_2)
            (:LoopBody
              (Variables|Default|Setset_item true)
              (if (== (Utilities|Array|Length (Variables|Default|Getitem_check)) (Utilities|Array|Length (Variables|/Game/Blueprint/Primary_Data_Asset/BP_PDA_Symptome.BP_PDA_Symptome_C|Getlist_information _array_element_3)))
                (CallFunction|CheckItemCheckContains (Variables|/Game/Blueprint/Primary_Data_Asset/BP_PDA_Symptome.BP_PDA_Symptome_C|Getlist_information _array_element_3))
                (if (Variables|Default|Getset_item)
                  (if (Utilities|Enum|Equal(Enum) (Variables|/Game/Blueprint/Primary_Data_Asset/BP_PDA_Item.BP_PDA_Item_C|Getmemory (Utilities|Array|Get(acopy) _list_symptome _array_index_2)) "NewEnumerator0")
                    (Variables|Default|Setitem_to_out (Utilities|Array|Get(acopy) _list_symptome _array_index_2))
                    (goto _label_2 Break)))))
            (:Completed
              (Utilities|IsValid (Variables|Default|Getitem_to_out)
                (:Is%20Valid
                  (Development|PrintString "fusion symptome"))
                (:Is%20Not%20Valid
                  (Development|PrintString "echec fusion"))))))))))

(fn AddItemFusion
  (bind _asbp_first_person_player_controller (CallFunction|GetController))
  (bind _disc_05 (Variables|Default|Getdisc_05))
  (bind _disc_04 (Variables|Default|Getdisc_04))
  (bind _disc_03 (Variables|Default|Getdisc_03))
  (bind _disc_02 (Variables|Default|Getdisc_02))
  (bind _disc_01 (Variables|Default|Getdisc_01))
  (bind _selected_item (Variables|/Game/FirstPerson/Blueprints/BP_FirstPersonPlayerController.BP_FirstPersonPlayerController_C|Getselected_item _asbp_first_person_player_controller))
  (bind _inventory (Variables|/Game/FirstPerson/Blueprints/BP_FirstPersonPlayerController.BP_FirstPersonPlayerController_C|Getinventory _asbp_first_person_player_controller))
  (bind _output (Utilities|Array|Get(acopy) _inventory _selected_item))
  (bind _mesh (Variables|/Game/Blueprint/Primary_Data_Asset/BP_PDA_Item.BP_PDA_Item_C|Getmesh _output))
  (bind _mesh_2 (Variables|/Game/Blueprint/Primary_Data_Asset/BP_PDA_Item.BP_PDA_Item_C|Getmesh _output))
  (if (< (Utilities|Array|Length (Variables|Default|Getitem_fusion)) (Variables|Default|Getmax_item))
    (bind _returnvalue (Utilities|Array|Add (Variables|Default|Getitem_fusion) _output))
    (switch int _returnvalue
      (:0
        (Components|StaticMesh|SetStaticMesh _disc_01 _mesh_2)
        (Rendering|SetVisibility _disc_01 true false))
      (:1
        (Components|StaticMesh|SetStaticMesh _disc_02 _mesh_2)
        (Rendering|SetVisibility _disc_02 true false))
      (:2
        (Components|StaticMesh|SetStaticMesh _disc_03 _mesh)
        (Rendering|SetVisibility _disc_03 true false))
      (:3
        (Components|StaticMesh|SetStaticMesh _disc_04 _mesh)
        (Rendering|SetVisibility _disc_04 true false))
      (:4
        (Components|StaticMesh|SetStaticMesh _disc_05 (Variables|/Game/Blueprint/Primary_Data_Asset/BP_PDA_Item.BP_PDA_Item_C|Getmesh _output))
        (Rendering|SetVisibility _disc_05 true false)))
    (Components|Animation|PlayAnimation (Variables|/Game/FirstPerson/Blueprints/BP_FirstPersonCharacter.BP_FirstPersonCharacter_C|GetArm (CallFunction|GetCharacter)) "/Game/Mesh/Arm/Animations/Hide/AS_Bras_Hide.AS_Bras_Hide" false)
    (Default|InventoryRemove _asbp_first_person_player_controller)))

(fn SymptometoInformation
  (if (Utilities|Array|IsNotEmpty (Variables|Default|Getitem_check))
    (Utilities|Array|Clear (Variables|Default|Getitem_check)))
  (for _array_element (Variables|Default|Getitem_fusion)
    (bind _asbp_pda_information (Utilities|Casting|CastToBP_PDA_Information _array_element)
      (:then
        (Utilities|Array|Add (Variables|Default|Getitem_check) _asbp_pda_information))
      (:CastFailed
        (bind _asbp_pda_symptome (Utilities|Casting|CastToBP_PDA_Symptome _array_element))
        (for _array_element_2 (Variables|/Game/Blueprint/Primary_Data_Asset/BP_PDA_Symptome.BP_PDA_Symptome_C|Getlist_information _asbp_pda_symptome)
          (Utilities|Array|Add (Variables|Default|Getitem_check) _array_element_2))))))

(fn AddInfoDiag
  (params (list_inormation :type Array%20of%20BP%20PDA%20Information%20Object%20References))
  (for _array_element list_inormation
    (Utilities|Array|Add (Variables|Default|Getinfo_diag) _array_element)))

(fn CheckItemCheckContains
  (params (list_information :type Array%20of%20BP%20PDA%20Information%20Object%20References))
  (bind _array_element (Utilities|Array|ForEachLoopwithBreak list_information :!label _label)
    (:LoopBody
      (if (not (Utilities|Array|ContainsItem (Variables|Default|Getitem_check) _array_element))
        (Variables|Default|Setset_item false)
        (goto _label Break)))))

(fn ItemFusiontoInformationCheck
  (if (Utilities|Array|IsNotEmpty (Variables|Default|Getitem_fusion))
    (Utilities|Array|Clear (Variables|Default|Getitem_check))
    (for _array_element (Variables|Default|Getitem_fusion)
      (bind _asbp_pda_information (Utilities|Casting|CastToBP_PDA_Information _array_element)
        (:then
          (Utilities|Array|Add (Variables|Default|Getitem_check) _asbp_pda_information))
        (:CastFailed
          (bind _asbp_pda_symptome (Utilities|Casting|CastToBP_PDA_Symptome _array_element))
          (for _array_element_2 (Variables|/Game/Blueprint/Primary_Data_Asset/BP_PDA_Symptome.BP_PDA_Symptome_C|Getlist_information _asbp_pda_symptome)
            (Utilities|Array|Add (Variables|Default|Getitem_check) _array_element_2)))))
    (else
      (Development|PrintString "fusion vide"))))