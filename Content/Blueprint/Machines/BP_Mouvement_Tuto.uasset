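; BP_Mouvement_Tuto is a movement machine, apparently the tutorial variant, that spawns its own control panel on BeginPlay.
; SetPositions gathers placeholder components into info switch, member switch (head, body, limbs) and button arrays.
; Spawn creates switches, movement buttons and a validation button there, rotating relative locations by the actor's rotation and adding only its yaw to their rotations.
; Interract is empty, and CreateItem only calls the parent.
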(event EventBeginPlay
  (|CallParentFunction)
  (CallFunction|SetPositions)
  (CallFunction|Spawn))

(event Collision|EventActorBeginOverlap
  (params (OtherActor :type Actor%20Object%20Reference))
  (|CallParentFunction OtherActor) ; This node is disabled and will not be called.\nDrag off pins to build functionality.
)

(event EventTick
  (params (DeltaSeconds :type Float%20%28single-precision%29))
  (|CallParentFunction DeltaSeconds))

(fn ConstructionScript
  (|CallParentFunction))

(fn CreateItem
  (|CallParentFunction))

(fn SetInfoSwitchPosition
  (bind _info_switch_position (Variables|Default|Getinfo_switch_position))
  (Utilities|Array|Add _info_switch_position (Variables|Default|Getswitch_1))
  (Utilities|Array|Add _info_switch_position (Variables|Default|Getswitch_2))
  (Utilities|Array|Add _info_switch_position (Variables|Default|Getswitch_3))
  (Utilities|Array|Add _info_switch_position (Variables|Default|Getswitch_4))
  (Utilities|Array|Add _info_switch_position (Variables|Default|Getswitch_5)))

(fn SetMemberSwitchPosition
  (bind _member_switch_position (Variables|Default|Getmember_switch_position))
  (Utilities|Array|Add _member_switch_position (Variables|Default|Getswitch_Head))
  (Utilities|Array|Add _member_switch_position (Variables|Default|Getswitch_Body))
  (Utilities|Array|Add _member_switch_position (Variables|Default|Getswitch_BD))
  (Utilities|Array|Add _member_switch_position (Variables|Default|Getswitch_BG))
  (Utilities|Array|Add _member_switch_position (Variables|Default|Getswitch_JD))
  (Utilities|Array|Add _member_switch_position (Variables|Default|Getswitch_JG)))

(fn SetButtonPosition
  (bind _button_position (Variables|Default|Getbutton_position))
  (Utilities|Array|Add _button_position (Variables|Default|Getbutton_T))
  (Utilities|Array|Add _button_position (Variables|Default|Getbutton_C))
  (Utilities|Array|Add _button_position (Variables|Default|Getbutton_BD_1))
  (Utilities|Array|Add _button_position (Variables|Default|Getbutton_BD_2))
  (Utilities|Array|Add _button_position (Variables|Default|Getbutton_BD_3))
  (Utilities|Array|Add _button_position (Variables|Default|Getbutton_BG_1))
  (Utilities|Array|Add _button_position (Variables|Default|Getbutton_BG_2))
  (Utilities|Array|Add _button_position (Variables|Default|Getbutton_BG_3))
  (Utilities|Array|Add _button_position (Variables|Default|Getbutton_JD_1))
  (Utilities|Array|Add _button_position (Variables|Default|Getbutton_JD_2))
  (Utilities|Array|Add _button_position (Variables|Default|Getbutton_JD_3))
  (Utilities|Array|Add _button_position (Variables|Default|Getbutton_JG_1))
  (Utilities|Array|Add _button_position (Variables|Default|Getbutton_JG_2))
  (Utilities|Array|Add _button_position (Variables|Default|Getbutton_JG_3)))

(fn SetPositions
  (CallFunction|SetInfoSwitchPosition)
  (CallFunction|SetMemberSwitchPosition)
  (CallFunction|SetButtonPosition))

(fn Spawn
  (bind _returnvalue (Transformation|GetActorRotation))
  (bind _returnvalue_2 (Transformation|GetActorRotation))
  (bind _returnvalue_3 (Transformation|GetActorRotation))
  (bind _returnvalue_4 (Transformation|GetActorRotation))
  (bind _validation (Variables|Default|Getvalidation))
  (bind _relativerotation (Variables|/Script/Engine.SceneComponent|GetRelativeRotation _validation))
  (bind (_roll _pitch _yaw) (Math|Rotator|BreakRotator _relativerotation))
  (for _array_element (Variables|Default|Getinfo_switch_position)
    (Game|SpawnActorfromClass "/Game/Blueprint/Buttons/BP_Switch.BP_Switch_C" (Math|Transform|MakeTransform (+ (Math|Vector|RotateVector (Variables|/Script/Engine.SceneComponent|GetRelativeLocation _array_element) _returnvalue_2) (Transformation|GetActorLocation)) (Math|Rotator|MakeRotator (.Roll (Math|Rotator|BreakRotator (Variables|/Script/Engine.SceneComponent|GetRelativeRotation _array_element))) (.Pitch (Math|Rotator|BreakRotator (Variables|/Script/Engine.SceneComponent|GetRelativeRotation _array_element))) (+ (.Yaw (Math|Rotator|BreakRotator (Variables|/Script/Engine.SceneComponent|GetRelativeRotation _array_element))) (.Yaw (Math|Rotator|BreakRotator _returnvalue_2)))) "1.000000,1.000000,1.000000") "Undefined" "MultiplyWithRoot" 0 0))
  (for _array_element_2 (Variables|Default|Getmember_switch_position)
    (Game|SpawnActorfromClass "/Game/Blueprint/Buttons/BP_Switch.BP_Switch_C" (Math|Transform|MakeTransform (+ (Math|Vector|RotateVector (Variables|/Script/Engine.SceneComponent|GetRelativeLocation _array_element_2) _returnvalue_3) (Transformation|GetActorLocation)) (Math|Rotator|MakeRotator (.Roll (Math|Rotator|BreakRotator (Variables|/Script/Engine.SceneComponent|GetRelativeRotation _array_element_2))) (.Pitch (Math|Rotator|BreakRotator (Variables|/Script/Engine.SceneComponent|GetRelativeRotation _array_element_2))) (+ (.Yaw (Math|Rotator|BreakRotator (Variables|/Script/Engine.SceneComponent|GetRelativeRotation _array_element_2))) (.Yaw (Math|Rotator|BreakRotator _returnvalue_3)))) "1.000000,1.000000,1.000000") "Undefined" "MultiplyWithRoot" 0 0))
  (for _array_element_3 (Variables|Default|Getbutton_position)
    (Game|SpawnActorfromClass "/Game/Blueprint/Buttons/BP_Mouvement_Button.BP_Mouvement_Button_C" (Math|Transform|MakeTransform (+ (Math|Vector|RotateVector (Variables|/Script/Engine.SceneComponent|GetRelativeLocation _array_element_3) _returnvalue_4) (Transformation|GetActorLocation)) (Math|Rotator|MakeRotator (.Roll (Math|Rotator|BreakRotator (Variables|/Script/Engine.SceneComponent|GetRelativeRotation _array_element_3))) (.Pitch (Math|Rotator|BreakRotator (Variables|/Script/Engine.SceneComponent|GetRelativeRotation _array_element_3))) (+ (.Yaw (Math|Rotator|BreakRotator (Variables|/Script/Engine.SceneComponent|GetRelativeRotation _array_element_3))) (.Yaw (Math|Rotator|BreakRotator _returnvalue_4)))) "1.000000,1.000000,1.000000") "Undefined" "MultiplyWithRoot" 0 0))
  (Game|SpawnActorfromClass "/Game/Blueprint/Buttons/BP_Button.BP_Button_C" (Math|Transform|MakeTransform (+ (Math|Vector|RotateVector (Variables|/Script/Engine.SceneComponent|GetRelativeLocation _validation) _returnvalue) (Transformation|GetActorLocation)) (Math|Rotator|MakeRotator _roll _pitch (+ _yaw (.Yaw (Math|Rotator|BreakRotator _returnvalue)))) "1.000000,1.000000,1.000000") "Undefined" "MultiplyWithRoot" 0 0))

(fn Interract)