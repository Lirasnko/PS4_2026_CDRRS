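; Memory machine that takes a floppy disk from the player and outputs the entry of the same Type stored in BP_Generate's Memory.
; Interacting moves the selected inventory item into the machine, or advances the tutorial once when the selected slot is empty.
; CreateItem spawns a BP_Item at the rotated Output point, passing the input through when Memory is empty or no match is found, then clears the input.
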(event EventBeginPlay
  (bind _widget (Variables|Default|GetWidget))
  (bind _returnvalue (UserInterface|GetUserWidgetObject _widget))
  (|CallParentFunction)
  (bind _aswbp_memory (Utilities|Casting|CastToWBP_Memory _returnvalue))
  (Variables|/Game/Widget/WBP_Memory.WBP_Memory_C|Setmachine_ref _aswbp_memory self)
  (Variables|Default|Setmachine_ui _returnvalue))

(fn ConstructionScript
  (|CallParentFunction))

(fn Interract
  (bind _asbp_first_person_player_controller (CallFunction|GetController))
  (bind _selected_item (Variables|/Game/FirstPerson/Blueprints/BP_FirstPersonPlayerController.BP_FirstPersonPlayerController_C|Getselected_item _asbp_first_person_player_controller))
  (bind _inventory (Variables|/Game/FirstPerson/Blueprints/BP_FirstPersonPlayerController.BP_FirstPersonPlayerController_C|Getinventory _asbp_first_person_player_controller))
  (bind _output (Utilities|Array|Get(acopy) _inventory _selected_item))
  (|CallParentFunction)
  (Variables|Default|Getinput_floppydisk
    (:then)
    (:else
      (if (!= _output "/Game/Data_Asset/DA_Item_Void.DA_Item_Void")
        (Variables|Default|Setinput_floppydisk _output)
        (Utilities|Array|Insert _inventory "/Game/Data_Asset/DA_Item_Void.DA_Item_Void" _selected_item)
        (Utilities|Array|RemoveIndex _inventory (+ _selected_item 1))
        (Default|SetIcons (Variables|/Game/FirstPerson/Blueprints/BP_FirstPersonPlayerController.BP_FirstPersonPlayerController_C|Getin_game_ui _asbp_first_person_player_controller))
        (else
          (Development|PrintString "false")
          (bind _returnvalue (Actor|GetActorOfClass "/Game/Blueprint/BP_Generate.BP_Generate_C"))
          (if (Variables|/Game/Blueprint/BP_Generate.BP_Generate_C|Gettuto _returnvalue)
            (if (Variables|Default|Gettuto_done)
              (Development|PrintString "tuto done")
              (elif (Variables|/Game/FirstPerson/Blueprints/BP_FirstPersonPlayerController.BP_FirstPersonPlayerController_C|Getis_interacting (CallFunction|GetController))
                (Development|PrintString "interacting")
                (else
                  (bind _returnvalue_2 (Actor|GetActorOfClass "/Game/Blueprint/BP_Tuto.BP_Tuto_C"))
                  (Default|UpdateText _returnvalue_2)
                  (Default|Lighton _returnvalue_2 "Fusion_light" "Memory_light")
                  (Default|Lighton _returnvalue_2 "Move_light" "")
                  (Variables|Default|Settuto_done true))))))))))

(fn CreateItem
  (bind _returnvalue (Transformation|GetActorLocation))
  (bind _returnvalue_2 (Transformation|GetActorRotation))
  (bind _output (Variables|Default|GetOutput))
  (bind _yaw (Math|Rotator|BreakRotator _returnvalue_2))
  (bind _relativelocation (Variables|/Script/Engine.SceneComponent|GetRelativeLocation _output))
  (bind _relativerotation (Variables|/Script/Engine.SceneComponent|GetRelativeRotation _output))
  (bind (_roll _pitch _yaw_2) (Math|Rotator|BreakRotator _relativerotation))
  (bind _returnvalue_3 (Math|Vector|RotateVector _relativelocation _returnvalue_2))
  (bind _returnvalue_4 (+ _pitch 9e+01))
  (bind _returnvalue_5 (+ _roll _yaw 9e+01))
  (bind _returnvalue_6 (+ _returnvalue_3 _returnvalue))
  (bind _returnvalue_7 (Math|Rotator|MakeRotator _returnvalue_4 _yaw_2 _returnvalue_5))
  (|CallParentFunction)
  (bind _returnvalue_8 (Actor|GetActorOfClass "/Game/Blueprint/BP_Generate.BP_Generate_C"))
  (if (Utilities|Array|IsEmpty (Variables|/Game/Blueprint/BP_Generate.BP_Generate_C|Getmemory _returnvalue_8))
    (bind _returnvalue_9 (Game|SpawnActorfromClass "/Game/Blueprint/BP_Item.BP_Item_C" (Math|Transform|MakeTransform _returnvalue_6 _returnvalue_7 "1.000000,1.000000,1.000000") "Undefined" "MultiplyWithRoot" 0 0))
    (Variables|/Game/Blueprint/BP_Item.BP_Item_C|Setitem _returnvalue_9 (Variables|Default|Getinput_floppydisk))
    (Default|SetMesh _returnvalue_9)
    (Variables|Default|Setinput_floppydisk 0 :!label _label)
    (else
      (bind _array_element (Utilities|Array|ForEachLoopwithBreak (Variables|/Game/Blueprint/BP_Generate.BP_Generate_C|Getmemory _returnvalue_8) :!label _label_2)
        (:LoopBody
          (if (Utilities|Enum|Equal(Enum) (Variables|/Game/Blueprint/Primary_Data_Asset/BP_PDA_Item.BP_PDA_Item_C|Gettype (Variables|Default|Getinput_floppydisk)) (Variables|/Game/Blueprint/Primary_Data_Asset/BP_PDA_Item.BP_PDA_Item_C|Gettype _array_element))
            (Variables|Default|Setoutput_floppydisk _array_element)
            (goto _label_2 Break)))
        (:Completed
          (Variables|Default|Getoutput_floppydisk
            (:then
              (bind _returnvalue_10 (Game|SpawnActorfromClass "/Game/Blueprint/BP_Item.BP_Item_C" (Math|Transform|MakeTransform _returnvalue_6 _returnvalue_7 "1.000000,1.000000,1.000000") "Undefined" "MultiplyWithRoot" 0 0))
              (Variables|/Game/Blueprint/BP_Item.BP_Item_C|Setitem _returnvalue_10 (Variables|Default|Getoutput_floppydisk))
              (Default|SetMesh _returnvalue_10)
              (goto _label))
            (:else
              (bind _returnvalue_11 (Game|SpawnActorfromClass "/Game/Blueprint/BP_Item.BP_Item_C" (Math|Transform|MakeTransform _returnvalue_6 _returnvalue_7 "1.000000,1.000000,1.000000") "Undefined" "MultiplyWithRoot" 0 0))
              (Variables|/Game/Blueprint/BP_Item.BP_Item_C|Setitem _returnvalue_11 (Variables|Default|Getinput_floppydisk))
              (Default|SetMesh _returnvalue_11)
              (goto _label))))))))

(fn CreateOrder)