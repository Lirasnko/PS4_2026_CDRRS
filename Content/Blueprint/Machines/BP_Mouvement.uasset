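; BP_Mouvement is a machine where switch settings for movement info and body members determine whether an item is produced.
; BeginPlay spawns info and member switches, per-segment movement buttons and a validation button at component positions, rotated with the actor.
; CreateItem checks switch booleans against ItemOut, spawning an unfound BP_Item, recording it on the controller and setting the alarm-off material.
; The InfoBool[4]-only branch spawns nothing, and Animation is an empty switch.
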(event EventBeginPlay
  (|CallParentFunction)
  (CallFunction|SetPositions)
  (CallFunction|Spawn))

(event Collision|EventActorBeginOverlap
  (params (OtherActor :type Actor%20Object%20Reference))
  (|CallParentFunction OtherActor) ; This node is disabled and will not be called.\nDrag off pins to build functionality.
)

(event EventTick
  (params (DeltaSeconds :type Float%20%28single-precision%29))
  (|CallParentFunction DeltaSeconds) ; This node is disabled and will not be called.\nDrag off pins to build functionality.
)

(fn ConstructionScript
  (|CallParentFunction))

(fn CreateItem
  (bind _returnvalue (Transformation|GetActorRotation))
  (bind _info_bool (Variables|Default|Getinfo_bool))
  (bind _info_bool_2 (Variables|Default|Getinfo_bool))
  (bind _info_bool_3 (Variables|Default|Getinfo_bool))
  (bind _item_out (Variables|Default|Getitem_out))
  (bind _item_out_2 (Variables|Default|Getitem_out))
  (bind _item_out_3 (Variables|Default|Getitem_out))
  (bind _item_out_4 (Variables|Default|Getitem_out))
  (bind _item_out_5 (Variables|Default|Getitem_out))
  (bind _item_out_6 (Variables|Default|Getitem_out))
  (bind _item_out_7 (Variables|Default|Getitem_out))
  (bind _item_out_8 (Variables|Default|Getitem_out))
  (bind _item_out_9 (Variables|Default|Getitem_out))
  (bind _item_out_10 (Variables|Default|Getitem_out))
  (bind _item_out_11 (Variables|Default|Getitem_out))
  (bind _item_out_12 (Variables|Default|Getitem_out))
  (bind _item_out_13 (Variables|Default|Getitem_out))
  (bind _item_out_14 (Variables|Default|Getitem_out))
  (bind _item_out_15 (Variables|Default|Getitem_out))
  (bind _item_out_16 (Variables|Default|Getitem_out))
  (bind _item_out_17 (Variables|Default|Getitem_out))
  (bind _item_out_18 (Variables|Default|Getitem_out))
  (bind _item_out_19 (Variables|Default|Getitem_out))
  (bind _item_out_20 (Variables|Default|Getitem_out))
  (bind _item_out_21 (Variables|Default|Getitem_out))
  (bind _item_out_22 (Variables|Default|Getitem_out))
  (bind _item_out_23 (Variables|Default|Getitem_out))
  (bind _output (Variables|Default|Getoutput))
  (bind _item_out_24 (Variables|Default|Getitem_out))
  (bind _item_out_25 (Variables|Default|Getitem_out))
  (bind _output_2 (Utilities|Array|Get(acopy) _info_bool 2))
  (bind _output_3 (Utilities|Array|Get(acopy) _info_bool_2 4))
  (bind _output_4 (Utilities|Array|Get(acopy) _info_bool_3 4))
  (bind _relativerotation (Variables|/Script/Engine.SceneComponent|GetRelativeRotation _output))
  (bind (_roll _pitch _yaw) (Math|Rotator|BreakRotator _relativerotation))
  (|CallParentFunction)
  (if (Utilities|Array|Get(acopy) (Variables|Default|Getinfo_bool) 3)
    (if (== (Variables|Default|Getitem_out) "/Game/Data_Asset/Information/Mouvement/DA_Info_MO_N.DA_Info_MO_N")
      (if (not (Utilities|Array|ContainsItem (Variables|/Game/FirstPerson/Blueprints/BP_FirstPersonPlayerController.BP_FirstPersonPlayerController_C|Getitem_find (CallFunction|GetController)) (Variables|Default|Getitem_out))) :!label _label
        (bind _returnvalue_2 (Game|SpawnActorfromClass "/Game/Blueprint/BP_Item.BP_Item_C" (Math|Transform|MakeTransform (+ (Math|Vector|RotateVector (Variables|/Script/Engine.SceneComponent|GetRelativeLocation _output) _returnvalue) (Transformation|GetActorLocation)) (Math|Rotator|MakeRotator (+ _pitch -9e+01) _yaw (+ _roll (.Yaw (Math|Rotator|BreakRotator _returnvalue)) 9e+01)) "1.000000,1.000000,1.000000") "Undefined" "MultiplyWithRoot" 0 0))
        (Variables|/Game/Blueprint/BP_Item.BP_Item_C|Setitem _returnvalue_2 _item_out_25)
        (Default|SetMesh _returnvalue_2)
        (Utilities|Array|Add (Variables|/Game/FirstPerson/Blueprints/BP_FirstPersonPlayerController.BP_FirstPersonPlayerController_C|Getitem_find (CallFunction|GetController)) _item_out_25)
        (Rendering|Material|SetMaterial (Variables|Default|Getlight) 0 "/Game/Materials/Boutons/Alarm/MI_Alarm_Off.MI_Alarm_Off")))
    (elif (Utilities|Array|Get(acopy) (Variables|Default|Getinfo_bool) 1)
      (for (_array_element _array_index) (Variables|Default|Getmember_bool)
        (if _array_element
          (switch int _array_index
            (:0
              (if (== _item_out "/Game/Data_Asset/Information/Mouvement/Tete/DA_Info_MO_P_T.DA_Info_MO_P_T")
                (goto _label)))
            (:1
              (if (== _item_out "/Game/Data_Asset/Information/Mouvement/Corp/DA_Info_MO_P_C.DA_Info_MO_P_C")
                (goto _label)))
            (:2
              (if (== _item_out_2 "/Game/Data_Asset/Information/Mouvement/Bras_Droit/DA_Info_MO_P_BD.DA_Info_MO_P_BD")
                (goto _label)))
            (:3
              (if (== _item_out_2 "/Game/Data_Asset/Information/Mouvement/Bras_Gauche/DA_Info_MO_P_BG.DA_Info_MO_P_BG")
                (goto _label)))
            (:4
              (if (== _item_out_3 "/Game/Data_Asset/Information/Mouvement/Jambe_Droite/DA_Info_MO_P_JD.DA_Info_MO_P_JD")
                (goto _label)))
            (:5
              (if (== _item_out_3 "/Game/Data_Asset/Information/Mouvement/Jambe_Gauche/DA_Info_MO_P_JG.DA_Info_MO_P_JG")
                (goto _label))))))
      (elif (Utilities|Array|Get(acopy) (Variables|Default|Getinfo_bool))
        (if _output_2
          (if _output_3
            (for (_array_element_2 _array_index_2) (Variables|Default|Getmember_bool)
              (if _array_element_2
                (switch int _array_index_2
                  (:0
                    (if (== _item_out_13 "/Game/Data_Asset/Information/Mouvement/Tete/DA_Info_MO_L_D_A_T.DA_Info_MO_L_D_A_T")
                      (goto _label)))
                  (:1
                    (if (== _item_out_13 "/Game/Data_Asset/Information/Mouvement/Corp/DA_Info_MO_L_D_A_C.DA_Info_MO_L_D_A_C")
                      (goto _label)))
                  (:2
                    (if (== _item_out_14 "/Game/Data_Asset/Information/Mouvement/Bras_Droit/DA_Info_MO_L_D_A_BD.DA_Info_MO_L_D_A_BD")
                      (goto _label)))
                  (:3
                    (if (== _item_out_14 "/Game/Data_Asset/Information/Mouvement/Bras_Gauche/DA_Info_MO_L_D_A_BG.DA_Info_MO_L_D_A_BG")
                      (goto _label)))
                  (:4
                    (if (== _item_out_15 "/Game/Data_Asset/Information/Mouvement/Jambe_Droite/DA_Info_MO_L_D_A_JD.DA_Info_MO_L_D_A_JD")
                      (goto _label)))
                  (:5
                    (if (== _item_out_15 "/Game/Data_Asset/Information/Mouvement/Jambe_Gauche/DA_Info_MO_L_D_A_JG.DA_Info_MO_L_D_A_JG")
                      (goto _label))))))
            (else
              (for (_array_element_3 _array_index_3) (Variables|Default|Getmember_bool)
                (if _array_element_3
                  (switch int _array_index_3
                    (:0
                      (if (== _item_out_16 "/Game/Data_Asset/Information/Mouvement/Tete/DA_Info_MO_D_A_T.DA_Info_MO_D_A_T")
                        (goto _label)))
                    (:1
                      (if (== _item_out_16 "/Game/Data_Asset/Information/Mouvement/Corp/DA_Info_MO_D_A_C.DA_Info_MO_D_A_C")
                        (goto _label)))
                    (:2
                      (if (== _item_out_17 "/Game/Data_Asset/Information/Mouvement/Bras_Droit/DA_Info_MO_D_A_BD.DA_Info_MO_D_A_BD")
                        (goto _label)))
                    (:3
                      (if (== _item_out_17 "/Game/Data_Asset/Information/Mouvement/Bras_Gauche/DA_Info_MO_D_A_BG.DA_Info_MO_D_A_BG")
                        (goto _label)))
                    (:4
                      (if (== _item_out_18 "/Game/Data_Asset/Information/Mouvement/Jambe_Droite/DA_Info_MO_D_A_JD.DA_Info_MO_D_A_JD")
                        (goto _label)))
                    (:5
                      (if (== _item_out_18 "/Game/Data_Asset/Information/Mouvement/Jambe_Gauche/DA_Info_MO_D_A_JG.DA_Info_MO_D_A_JG")
                        (goto _label))))))))
          (elif _output_3
            (for (_array_element_4 _array_index_4) (Variables|Default|Getmember_bool)
              (if _array_element_4
                (switch int _array_index_4
                  (:0
                    (if (== _item_out_19 "/Game/Data_Asset/Information/Mouvement/Tete/DA_Info_MO_L_A_T.DA_Info_MO_L_A_T")
                      (goto _label)))
                  (:1
                    (if (== _item_out_19 "/Game/Data_Asset/Information/Mouvement/Corp/DA_Info_MO_L_A_C.DA_Info_MO_L_A_C")
                      (goto _label)))
                  (:2
                    (if (== _item_out_20 "/Game/Data_Asset/Information/Mouvement/Bras_Droit/DA_Info_MO_L_A_BD.DA_Info_MO_L_A_BD")
                      (goto _label)))
                  (:3
                    (if (== _item_out_20 "/Game/Data_Asset/Information/Mouvement/Bras_Gauche/DA_Info_MO_L_A_BG.DA_Info_MO_L_A_BG")
                      (goto _label)))
                  (:4
                    (if (== _item_out_21 "/Game/Data_Asset/Information/Mouvement/Jambe_Droite/DA_Info_MO_L_A_JD.DA_Info_MO_L_A_JD")
                      (goto _label)))
                  (:5
                    (if (== _item_out_21 "/Game/Data_Asset/Information/Mouvement/Jambe_Gauche/DA_Info_MO_L_A_JG.DA_Info_MO_L_A_JG")
                      (goto _label))))))
            (else
              (for (_array_element_5 _array_index_5) (Variables|Default|Getmember_bool)
                (if _array_element_5
                  (switch int _array_index_5
                    (:0
                      (if (== _item_out_22 "/Game/Data_Asset/Information/Mouvement/Tete/DA_Info_MO_A_T.DA_Info_MO_A_T")
                        (goto _label)))
                    (:1
                      (if (== _item_out_22 "/Game/Data_Asset/Information/Mouvement/Corp/DA_Info_MO_A_C.DA_Info_MO_A_C")
                        (goto _label)))
                    (:2
                      (if (== _item_out_23 "/Game/Data_Asset/Information/Mouvement/Bras_Droit/DA_Info_MO_A_BD.DA_Info_MO_A_BD")
                        (goto _label)))
                    (:3
                      (if (== _item_out_23 "/Game/Data_Asset/Information/Mouvement/Bras_Gauche/DA_Info_MO_A_BG.DA_Info_MO_A_BG")
                        (goto _label)))
                    (:4
                      (if (== _item_out_24 "/Game/Data_Asset/Information/Mouvement/Jambe_Droite/DA_Info_MO_A_JD.DA_Info_MO_A_JD")
                        (goto _label)))
                    (:5
                      (if (== _item_out_24 "/Game/Data_Asset/Information/Mouvement/Jambe_Gauche/DA_Info_MO_A_JG.DA_Info_MO_A_JG")
                        (goto _label)))))))))
        (elif _output_2
          (if _output_4
            (for (_array_element_6 _array_index_6) (Variables|Default|Getmember_bool)
              (if _array_element_6
                (switch int _array_index_6
                  (:0
                    (if (== _item_out_7 "/Game/Data_Asset/Information/Mouvement/Tete/DA_Info_MO_L_D_T.DA_Info_MO_L_D_T")
                      (goto _label)))
                  (:1
                    (if (== _item_out_7 "/Game/Data_Asset/Information/Mouvement/Corp/DA_Info_MO_L_D_C.DA_Info_MO_L_D_C")
                      (goto _label)))
                  (:2
                    (if (== _item_out_8 "/Game/Data_Asset/Information/Mouvement/Bras_Droit/DA_Info_MO_L_D_BD.DA_Info_MO_L_D_BD")
                      (goto _label)))
                  (:3
                    (if (== _item_out_8 "/Game/Data_Asset/Information/Mouvement/Bras_Gauche/DA_Info_MO_L_D_BG.DA_Info_MO_L_D_BG")
                      (goto _label)))
                  (:4
                    (if (== _item_out_9 "/Game/Data_Asset/Information/Mouvement/Jambe_Droite/DA_Info_MO_L_D_JD.DA_Info_MO_L_D_JD")
                      (goto _label)))
                  (:5
                    (if (== _item_out_9 "/Game/Data_Asset/Information/Mouvement/Jambe_Gauche/DA_Info_MO_L_D_JG.DA_Info_MO_L_D_JG")
                      (goto _label))))))
            (else
              (for (_array_element_7 _array_index_7) (Variables|Default|Getmember_bool)
                (if _array_element_7
                  (switch int _array_index_7
                    (:0
                      (if (== _item_out_10 "/Game/Data_Asset/Information/Mouvement/Tete/DA_Info_MO_D_T.DA_Info_MO_D_T")
                        (goto _label)))
                    (:1
                      (if (== _item_out_10 "/Game/Data_Asset/Information/Mouvement/Corp/DA_Info_MO_D_C.DA_Info_MO_D_C")
                        (goto _label)))
                    (:2
                      (if (== _item_out_11 "/Game/Data_Asset/Information/Mouvement/Bras_Droit/DA_Info_MO_D_BD.DA_Info_MO_D_BD")
                        (goto _label)))
                    (:3
                      (if (== _item_out_11 "/Game/Data_Asset/Information/Mouvement/Bras_Gauche/DA_Info_MO_D_BG.DA_Info_MO_D_BG")
                        (goto _label)))
                    (:4
                      (if (== _item_out_12 "/Game/Data_Asset/Information/Mouvement/Jambe_Droite/DA_Info_MO_D_JD.DA_Info_MO_D_JD")
                        (goto _label)))
                    (:5
                      (if (== _item_out_12 "/Game/Data_Asset/Information/Mouvement/Jambe_Gauche/DA_Info_MO_D_JG.DA_Info_MO_D_JG")
                        (goto _label))))))))
          (elif _output_4
            (for (_array_element_8 _array_index_8) (Variables|Default|Getmember_bool)
              (if _array_element_8
                (switch int _array_index_8
                  (:0
                    (if (== _item_out_4 "/Game/Data_Asset/Information/Mouvement/Tete/DA_Info_MO_L_T.DA_Info_MO_L_T")
                      _))
                  (:1
                    (if (== _item_out_4 "/Game/Data_Asset/Information/Mouvement/Corp/DA_Info_MO_L_C.DA_Info_MO_L_C")
                      _))
                  (:2
                    (if (== _item_out_5 "/Game/Data_Asset/Information/Mouvement/Bras_Droit/DA_Info_MO_L_BD.DA_Info_MO_L_BD")
                      _))
                  (:3
                    (if (== _item_out_5 "/Game/Data_Asset/Information/Mouvement/Bras_Gauche/DA_Info_MO_L_BG.DA_Info_MO_L_BG")
                      _))
                  (:4
                    (if (== _item_out_6 "/Game/Data_Asset/Information/Mouvement/Jambe_Droite/DA_Info_MO_L_JD.DA_Info_MO_L_JD")
                      _))
                  (:5
                    (if (== _item_out_6 "/Game/Data_Asset/Information/Mouvement/Jambe_Gauche/DA_Info_MO_L_JG.DA_Info_MO_L_JG")
                      _)))))))))))

(fn SetInfoSwitchPosition
  (bind _info_switch_position (Variables|Default|Getinfo_switch_position))
  (Utilities|Array|Add _info_switch_position (Variables|Default|Getswitch_1))
  (Utilities|Array|Add _info_switch_position (Variables|Default|Getswitch_2))
  (Utilities|Array|Add _info_switch_position (Variables|Default|Getswitch_3))
  (Utilities|Array|Add _info_switch_position (Variables|Default|Getswitch_4))
  (Utilities|Array|Add _info_switch_position (Variables|Default|Getswitch_5)))

(fn SetMemberSwitchPosition
  (bind _member_switch_position (Variables|Default|Getmember_switch_position))
  (Utilities|Array|Add _member_switch_position (Variables|Default|Getswitch_Head))
  (Utilities|Array|Add _member_switch_position (Variables|Default|Getswitch_Body))
  (Utilities|Array|Add _member_switch_position (Variables|Default|Getswitch_BD))
  (Utilities|Array|Add _member_switch_position (Variables|Default|Getswitch_BG))
  (Utilities|Array|Add _member_switch_position (Variables|Default|Getswitch_JD))
  (Utilities|Array|Add _member_switch_position (Variables|Default|Getswitch_JG)))

(fn SetButtonPosition
  (bind _button_position (Variables|Default|Getbutton_position))
  (Utilities|Array|Add _button_position (Variables|Default|Getbutton_T))
  (Utilities|Array|Add _button_position (Variables|Default|Getbutton_C))
  (Utilities|Array|Add _button_position (Variables|Default|Getbutton_BD_1))
  (Utilities|Array|Add _button_position (Variables|Default|Getbutton_BD_2))
  (Utilities|Array|Add _button_position (Variables|Default|Getbutton_BD_3))
  (Utilities|Array|Add _button_position (Variables|Default|Getbutton_BG_1))
  (Utilities|Array|Add _button_position (Variables|Default|Getbutton_BG_2))
  (Utilities|Array|Add _button_position (Variables|Default|Getbutton_BG_3))
  (Utilities|Array|Add _button_position (Variables|Default|Getbutton_JD_1))
  (Utilities|Array|Add _button_position (Variables|Default|Getbutton_JD_2))
  (Utilities|Array|Add _button_position (Variables|Default|Getbutton_JD_3))
  (Utilities|Array|Add _button_position (Variables|Default|Getbutton_JG_1))
  (Utilities|Array|Add _button_position (Variables|Default|Getbutton_JG_2))
  (Utilities|Array|Add _button_position (Variables|Default|Getbutton_JG_3)))

(fn SetPositions
  (CallFunction|SetInfoSwitchPosition)
  (CallFunction|SetMemberSwitchPosition)
  (CallFunction|SetButtonPosition))

(fn Spawn
  (bind _returnvalue (Transformation|GetActorRotation))
  (bind _returnvalue_2 (Transformation|GetActorRotation))
  (bind _returnvalue_3 (Transformation|GetActorRotation))
  (bind _returnvalue_4 (Transformation|GetActorRotation))
  (bind _info_switch_position (Variables|Default|Getinfo_switch_position))
  (bind _validation (Variables|Default|Getvalidation))
  (bind _relativerotation (Variables|/Script/Engine.SceneComponent|GetRelativeRotation _validation))
  (bind (_roll _pitch _yaw) (Math|Rotator|BreakRotator _relativerotation))
  (for (_array_element _array_index) _info_switch_position
    (bind _returnvalue_5 (Game|SpawnActorfromClass "/Game/Blueprint/Buttons/BP_Switch.BP_Switch_C" (Math|Transform|MakeTransform (+ (Math|Vector|RotateVector (Variables|/Script/Engine.SceneComponent|GetRelativeLocation _array_element) _returnvalue_2) (Transformation|GetActorLocation)) (Math|Rotator|MakeRotator (.Roll (Math|Rotator|BreakRotator (Variables|/Script/Engine.SceneComponent|GetRelativeRotation _array_element))) (.Pitch (Math|Rotator|BreakRotator (Variables|/Script/Engine.SceneComponent|GetRelativeRotation _array_element))) (+ (.Yaw (Math|Rotator|BreakRotator (Variables|/Script/Engine.SceneComponent|GetRelativeRotation _array_element))) (.Yaw (Math|Rotator|BreakRotator _returnvalue_2)))) "1.000000,1.000000,1.000000") "Undefined" "MultiplyWithRoot" 0 0))
    (Variables|/Game/Blueprint/Buttons/BP_Switch.BP_Switch_C|Setindex _returnvalue_5 _array_index)
    (Variables|/Game/Blueprint/Buttons/BP_Switch.BP_Switch_C|Setmachine_parent _returnvalue_5 self)
    (Utilities|Array|Add (Variables|Default|Getinfo_bool) false))
  (Utilities|Array|Clear (Variables|Default|Getmember_switch))
  (for (_array_element_2 _array_index_2) (Variables|Default|Getmember_switch_position)
    (bind _returnvalue_6 (Game|SpawnActorfromClass "/Game/Blueprint/Buttons/BP_Switch.BP_Switch_C" (Math|Transform|MakeTransform (+ (Math|Vector|RotateVector (Variables|/Script/Engine.SceneComponent|GetRelativeLocation _array_element_2) _returnvalue_3) (Transformation|GetActorLocation)) (Math|Rotator|MakeRotator (.Roll (Math|Rotator|BreakRotator (Variables|/Script/Engine.SceneComponent|GetRelativeRotation _array_element_2))) (.Pitch (Math|Rotator|BreakRotator (Variables|/Script/Engine.SceneComponent|GetRelativeRotation _array_element_2))) (+ (.Yaw (Math|Rotator|BreakRotator (Variables|/Script/Engine.SceneComponent|GetRelativeRotation _array_element_2))) (.Yaw (Math|Rotator|BreakRotator _returnvalue_3)))) "1.000000,1.000000,1.000000") "Undefined" "MultiplyWithRoot" 0 0))
    (Variables|/Game/Blueprint/Buttons/BP_Switch.BP_Switch_C|Setindex _returnvalue_6 (+ _array_index_2 (Utilities|Array|Length _info_switch_position)))
    (Variables|/Game/Blueprint/Buttons/BP_Switch.BP_Switch_C|Setmachine_parent _returnvalue_6 self)
    (Utilities|Array|Add (Variables|Default|Getmember_bool) false)
    (Utilities|Array|Add (Variables|Default|Getmember_switch) _returnvalue_6))
  (for (_array_element_3 _array_index_3) (Variables|Default|Getbutton_position)
    (bind _returnvalue_7 (Game|SpawnActorfromClass "/Game/Blueprint/Buttons/BP_Mouvement_Button.BP_Mouvement_Button_C" (Math|Transform|MakeTransform (+ (Math|Vector|RotateVector (Variables|/Script/Engine.SceneComponent|GetRelativeLocation _array_element_3) _returnvalue_4) (Transformation|GetActorLocation)) (Math|Rotator|MakeRotator (.Roll (Math|Rotator|BreakRotator (Variables|/Script/Engine.SceneComponent|GetRelativeRotation _array_element_3))) (.Pitch (Math|Rotator|BreakRotator (Variables|/Script/Engine.SceneComponent|GetRelativeRotation _array_element_3))) (+ (.Yaw (Math|Rotator|BreakRotator (Variables|/Script/Engine.SceneComponent|GetRelativeRotation _array_element_3))) (.Yaw (Math|Rotator|BreakRotator _returnvalue_4)))) "1.000000,1.000000,1.000000") "Undefined" "MultiplyWithRoot" 0 0))
    (Variables|/Game/Blueprint/Buttons/BP_Mouvement_Button.BP_Mouvement_Button_C|Setparent _returnvalue_7 self)
    (Variables|/Game/Blueprint/Buttons/BP_Mouvement_Button.BP_Mouvement_Button_C|Setindex _returnvalue_7 _array_index_3))
  (bind _returnvalue_8 (Game|SpawnActorfromClass "/Game/Blueprint/Buttons/BP_Button.BP_Button_C" (Math|Transform|MakeTransform (+ (Math|Vector|RotateVector (Variables|/Script/Engine.SceneComponent|GetRelativeLocation _validation) _returnvalue) (Transformation|GetActorLocation)) (Math|Rotator|MakeRotator _roll _pitch (+ _yaw (.Yaw (Math|Rotator|BreakRotator _returnvalue)))) "1.000000,1.000000,1.000000") "Undefined" "MultiplyWithRoot" 0 0))
  (Variables|/Game/Blueprint/Buttons/BP_Button.BP_Button_C|Setmachine_parent _returnvalue_8 self))

(fn SetPlane
  (bind _member (Variables|Default|Getmember))
  (Utilities|Array|Add _member (Variables|Default|Gethead))
  (Utilities|Array|Add _member (Variables|Default|Getbody))
  (Utilities|Array|Add _member (Variables|Default|GetBD_1))
  (Utilities|Array|Add _member (Variables|Default|GetBD_2))
  (Utilities|Array|Add _member (Variables|Default|GetBD_3))
  (Utilities|Array|Add _member (Variables|Default|GetBG_1))
  (Utilities|Array|Add _member (Variables|Default|GetBG_2))
  (Utilities|Array|Add _member (Variables|Default|GetBG_3))
  (Utilities|Array|Add _member (Variables|Default|GetJD_1))
  (Utilities|Array|Add _member (Variables|Default|GetJD_2))
  (Utilities|Array|Add _member (Variables|Default|GetJD_3))
  (Utilities|Array|Add _member (Variables|Default|GetJG_1))
  (Utilities|Array|Add _member (Variables|Default|GetJG_2))
  (Utilities|Array|Add _member (Variables|Default|GetJG_3)))

(fn Animation
  (params (index :type Integer))
  (switch int index))