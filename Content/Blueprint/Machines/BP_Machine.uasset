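; BP_Machine is a machine Blueprint that the player interacts with, switching the view between the pawn and the machine.
; Interract calls its parent, toggles character visibility, then blends the camera and flips the controller's IsInteracting flag while disabling or re-enabling character inputs.
; The character mesh hides immediately on entry and reappears after a delay on exit.
; CreateItem is an empty stub.
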(event Custom|toggleCharacterVisibility
  (bind _asbp_first_person_character (CallFunction|GetCharacter))
  (bind _mesh (Variables|/Script/Engine.Character|GetMesh _asbp_first_person_character))
  (if (Variables|/Game/FirstPerson/Blueprints/BP_FirstPersonPlayerController.BP_FirstPersonPlayerController_C|Getis_interacting (CallFunction|GetController))
    (Utilities|FlowControl|Delay 2.0)
    (Rendering|SetVisibility _mesh true true)
    (else
      (Rendering|SetVisibility _mesh false true))))

(event EventBeginPlay
  (|CallParentFunction) ; This node is disabled and will not be called.\nDrag off pins to build functionality.
)

(event Collision|EventActorBeginOverlap
  (params (OtherActor :type Actor%20Object%20Reference))
  (|CallParentFunction OtherActor) ; This node is disabled and will not be called.\nDrag off pins to build functionality.
)

(event EventTick
  (params (DeltaSeconds :type Float%20%28single-precision%29))
  (|CallParentFunction DeltaSeconds) ; This node is disabled and will not be called.\nDrag off pins to build functionality.
)

(fn ConstructionScript
  (|CallParentFunction))

(fn Interract
  (bind _asbp_first_person_player_controller (CallFunction|GetController))
  (bind _asbp_first_person_character (CallFunction|GetCharacter))
  (|CallParentFunction)
  (CallFunction|ToggleCharacterVisibility)
  (if (Variables|/Game/FirstPerson/Blueprints/BP_FirstPersonPlayerController.BP_FirstPersonPlayerController_C|Getis_interacting _asbp_first_person_player_controller)
    (Game|Player|SetViewTargetwithBlend _asbp_first_person_player_controller (Pawn|GetControlledPawn _asbp_first_person_player_controller) 0.5 "VTBlend_Linear" 0.0 false)
    (Variables|/Game/FirstPerson/Blueprints/BP_FirstPersonPlayerController.BP_FirstPersonPlayerController_C|Setis_interacting _asbp_first_person_player_controller false)
    (Default|EnableInputs _asbp_first_person_character)
    (else
      (Game|Player|SetViewTargetwithBlend _asbp_first_person_player_controller self 0.5 "VTBlend_Linear" 0.0 false)
      (Variables|/Game/FirstPerson/Blueprints/BP_FirstPersonPlayerController.BP_FirstPersonPlayerController_C|Setis_interacting _asbp_first_person_player_controller true)
      (Default|DisableInputs _asbp_first_person_character))))

(fn CreateItem)