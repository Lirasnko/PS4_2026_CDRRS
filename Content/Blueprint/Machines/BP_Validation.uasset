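; Validation machine where the player submits a diagnosis, checked against the DiagnostiqueToDo read from BP_Generate to end the game.
; Interact moves a selected diagnosis item from inventory into the machine, ignores symptom items and defers others to the parent.
; BeginPlay spawns a linked button at an arrow transform; EjectItem respawns the stored item.
; A correct validationCheck triggers confetti, blends to a menu camera, shows the end widget and sets IsOver.
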(event Custom|validationCheck
  (if (== (Variables|Default|Getvalidation) (Variables|Default|Getvalidation_check))
    (Niagara|SpawnSystematLocation "/Game/VFX/NS_Confetis_Burst.NS_Confetis_Burst" (Transformation|GetActorLocation))
    (bind _outactors (Actor|GetAllActorsOfClass "/Game/Blueprint/BP_MenuCamera.BP_MenuCamera_C"))
    (for _array_element _outactors
      (if (== (Variables|/Game/Blueprint/BP_MenuCamera.BP_MenuCamera_C|GetID _array_element) 5)
        (Game|Player|SetViewTargetwithBlend (CallFunction|GetController) _array_element 2.0 "VTBlend_Linear" 0.0 false)))
    (Utilities|FlowControl|Delay 2.0)
    (bind _returnvalue (UserInterface|CreateWidget "/Game/Widget/WBP_End.WBP_End_C"))
    (UserInterface|Viewport|AddtoViewport _returnvalue 0)
    (Utilities|FlowControl|Delay 1.0)
    (Variables|Default|Setis_over true)))

(event EventBeginPlay
  (Variables|Default|SetSKM true)
  (|CallParentFunction)
  (CallFunction|SpawnButton)
  (CallFunction|SetValidation))

(fn ConstructionScript
  (|CallParentFunction))

(fn CreateItem
  (|CallParentFunction))

(fn Interract
  (bind _asbp_first_person_player_controller (CallFunction|GetController))
  (bind _inventory (Variables|/Game/FirstPerson/Blueprints/BP_FirstPersonPlayerController.BP_FirstPersonPlayerController_C|Getinventory _asbp_first_person_player_controller))
  (bind _selected_item (Variables|/Game/FirstPerson/Blueprints/BP_FirstPersonPlayerController.BP_FirstPersonPlayerController_C|Getselected_item _asbp_first_person_player_controller))
  (bind _output (Utilities|Array|Get(acopy) _inventory _selected_item))
  (bind _asbp_pda_diagnostique (Utilities|Casting|CastToBP_PDA_Diagnostique _output)
    (:then
      (bind _output_get (Variables|Default|Setvalidation_check _asbp_pda_diagnostique))
      (Components|StaticMesh|SetStaticMesh (Variables|Default|Getitem) (Variables|/Game/Blueprint/Primary_Data_Asset/BP_PDA_Item.BP_PDA_Item_C|Getmesh _output_get))
      (Utilities|Array|Insert _inventory "/Game/Data_Asset/DA_Item_Void.DA_Item_Void" _selected_item)
      (Utilities|Array|RemoveIndex _inventory (+ _selected_item 1))
      (Default|SetIcons (Variables|/Game/FirstPerson/Blueprints/BP_FirstPersonPlayerController.BP_FirstPersonPlayerController_C|Getin_game_ui (CallFunction|GetController)))
      (Default|PlayAnimation (CallFunction|GetController) "/Game/Animations/Arm/AS_Arm_Throw_SoftHide.AS_Arm_Throw_SoftHide"))
    (:CastFailed
      (Utilities|Casting|CastToBP_PDA_Symptome _output
        (:CastFailed
          (|CallParentFunction))))))

(fn EjectItem
  (bind _returnvalue (Game|SpawnActorfromClass "/Game/Blueprint/BP_Item.BP_Item_C" (Math|Transform|MakeTransform "0, 0, 0" "0, 0, 0" "1.000000,1.000000,1.000000") "Undefined" "MultiplyWithRoot" 0 0))
  (Variables|/Game/Blueprint/BP_Item.BP_Item_C|Setitem _returnvalue (Variables|Default|Getvalidation_check)))

(fn SpawnButton
  (bind _returnvalue (Transformation|GetActorRotation))
  (bind _arrow_validation (Variables|Default|GetArrow_Validation))
  (bind _relativerotation (Variables|/Script/Engine.SceneComponent|GetRelativeRotation _arrow_validation))
  (bind (_roll _pitch _yaw) (Math|Rotator|BreakRotator _relativerotation))
  (bind _returnvalue_2 (Game|SpawnActorfromClass "/Game/Blueprint/Buttons/BP_Button_Validation.BP_Button_Validation_C" (Math|Transform|MakeTransform (+ (Math|Vector|RotateVector (Variables|/Script/Engine.SceneComponent|GetRelativeLocation _arrow_validation) _returnvalue) (Transformation|GetActorLocation)) (Math|Rotator|MakeRotator _roll _pitch (+ _yaw (.Yaw (Math|Rotator|BreakRotator _returnvalue)))) "1.000000,1.000000,1.000000") "Undefined" "MultiplyWithRoot" 0 0))
  (Variables|/Game/Blueprint/Buttons/BP_Button_Validation.BP_Button_Validation_C|Setmachine_parent _returnvalue_2 self))

(fn SetValidation
  (bind _returnvalue (Actor|GetActorOfClass "/Game/Blueprint/BP_Generate.BP_Generate_C"))
  (Variables|Default|Setvalidation (Variables|/Game/Blueprint/BP_Generate.BP_Generate_C|Getdiagnostique_to_do _returnvalue)))