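; BP_Screen is a machine that displays the icon of its output item and dispenses that item only if it has not been found yet.
; On BeginPlay it spawns a linked BP_Button and sets a dynamic M_Icon material to the item's sprite-sheet cell.
; CreateItem checks the controller's ItemFind list, then records the new item, spawns a BP_Item at the rotated output point, clears DoIt and updates the light.
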(event EventBeginPlay
  (bind _returnvalue (Transformation|GetActorRotation))
  (bind _button_position (Variables|Default|Getbutton_position))
  (bind _item_out (Variables|Default|Getitem_out))
  (bind _relativerotation (Variables|/Script/Engine.SceneComponent|GetRelativeRotation _button_position))
  (bind (_roll _pitch _yaw) (Math|Rotator|BreakRotator _relativerotation))
  (|CallParentFunction)
  (bind _returnvalue_2 (Game|SpawnActorfromClass "/Game/Blueprint/Buttons/BP_Button.BP_Button_C" (Math|Transform|MakeTransform (+ (Math|Vector|RotateVector (Variables|/Script/Engine.SceneComponent|GetRelativeLocation _button_position) _returnvalue) (Transformation|GetActorLocation)) (Math|Rotator|MakeRotator _roll _pitch (+ _yaw (.Yaw (Math|Rotator|BreakRotator _returnvalue)))) "1.000000,1.000000,1.000000") "Undefined" "MultiplyWithRoot" 0 0))
  (Variables|/Game/Blueprint/Buttons/BP_Button.BP_Button_C|Setmachine_parent _returnvalue_2 self)
  (bind _returnvalue_3 (Rendering|Material|CreateDynamicMaterialInstance (Variables|Default|Getscreen) 0 "/Game/Materials/M_Icon.M_Icon" "Icon" :!class /Script/Engine.PrimitiveComponent))
  (Rendering|Material|SetTextureParameterValue _returnvalue_3 "Sheet" (Variables|/Game/Blueprint/Primary_Data_Asset/BP_PDA_Item.BP_PDA_Item_C|Getsymbole _item_out))
  (Rendering|Material|SetScalarParameterValue _returnvalue_3 "grid_size" (Variables|/Game/Blueprint/Primary_Data_Asset/BP_PDA_Item.BP_PDA_Item_C|Getgrid_size _item_out) :!class /Script/Engine.MaterialInstanceDynamic)
  (Rendering|Material|SetScalarParameterValue _returnvalue_3 "colonne" (Variables|/Game/Blueprint/Primary_Data_Asset/BP_PDA_Item.BP_PDA_Item_C|Getcolonne _item_out) :!class /Script/Engine.MaterialInstanceDynamic)
  (Rendering|Material|SetScalarParameterValue _returnvalue_3 "ligne" (Variables|/Game/Blueprint/Primary_Data_Asset/BP_PDA_Item.BP_PDA_Item_C|Getligne _item_out) :!class /Script/Engine.MaterialInstanceDynamic))

(event Collision|EventActorBeginOverlap
  (params (OtherActor :type Actor%20Object%20Reference))
  (|CallParentFunction OtherActor) ; This node is disabled and will not be called.\nDrag off pins to build functionality.
)

(event EventTick
  (params (DeltaSeconds :type Float%20%28single-precision%29))
  (|CallParentFunction DeltaSeconds) ; This node is disabled and will not be called.\nDrag off pins to build functionality.
)

(fn ConstructionScript
  (|CallParentFunction))

(fn CreateItem
  (bind _returnvalue (Transformation|GetActorRotation))
  (bind _asbp_first_person_player_controller (CallFunction|GetController))
  (bind _item_out (Variables|Default|Getitem_out))
  (bind _output (Variables|Default|Getoutput))
  (bind _item_find (Variables|/Game/FirstPerson/Blueprints/BP_FirstPersonPlayerController.BP_FirstPersonPlayerController_C|Getitem_find _asbp_first_person_player_controller))
  (bind _relativerotation (Variables|/Script/Engine.SceneComponent|GetRelativeRotation _output))
  (bind (_roll _pitch _yaw) (Math|Rotator|BreakRotator _relativerotation))
  (|CallParentFunction)
  (if (not (Utilities|Array|ContainsItem _item_find _item_out))
    (Utilities|Array|Add _item_find _item_out)
    (bind _returnvalue_2 (Game|SpawnActorfromClass "/Game/Blueprint/BP_Item.BP_Item_C" (Math|Transform|MakeTransform (+ (Math|Vector|RotateVector (Variables|/Script/Engine.SceneComponent|GetRelativeLocation _output) _returnvalue) (Transformation|GetActorLocation)) (Math|Rotator|MakeRotator (+ _pitch 9e+01) _yaw (+ _roll (.Yaw (Math|Rotator|BreakRotator _returnvalue)) 9e+01)) "1.000000,1.000000,1.000000") "Undefined" "MultiplyWithRoot" 0 0))
    (Variables|/Game/Blueprint/BP_Item.BP_Item_C|Setitem _returnvalue_2 (Variables|Default|Getitem_out))
    (Default|SetMesh _returnvalue_2)
    (Variables|Default|Setdo_it false)
    (CallFunction|SetLight)))

(fn Interract
  (|CallParentFunction))