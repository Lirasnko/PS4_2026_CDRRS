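; BP_Fonction is a machine Blueprint that spawns a BP_Fonction_Line actor for the curve held in its Fonction variable.
; On BeginPlay it runs the parent logic, spawns the line at FonctionPos and copies Fonction.Curve into that actor.
; CreateItem and the construction script only call the parent, and CreateCurve is an empty stub.
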(event EventBeginPlay
  (|CallParentFunction)
  (bind _returnvalue (Game|SpawnActorfromClass "/Game/Blueprint/BP_Fonction_Line.BP_Fonction_Line_C" (Math|Transform|MakeTransform (Variables|Default|Getfonction_pos) "0, 0, 0" "1.000000,1.000000,1.000000") "Undefined" "MultiplyWithRoot" 0 0))
  (Variables|/Game/Blueprint/BP_Fonction_Line.BP_Fonction_Line_C|Setcurve _returnvalue (Variables|/Game/Blueprint/Primary_Data_Asset/BP_PDA_Fonction.BP_PDA_Fonction_C|Getcurve (Variables|Default|Getfonction))))

(event Collision|EventActorBeginOverlap
  (params (OtherActor :type Actor%20Object%20Reference))
  (|CallParentFunction OtherActor) ; This node is disabled and will not be called.\nDrag off pins to build functionality.
)

(event EventTick
  (params (DeltaSeconds :type Float%20%28single-precision%29))
  (|CallParentFunction DeltaSeconds) ; This node is disabled and will not be called.\nDrag off pins to build functionality.
)

(fn ConstructionScript
  (|CallParentFunction))

(fn CreateItem
  (|CallParentFunction))

(fn CreateCurve)