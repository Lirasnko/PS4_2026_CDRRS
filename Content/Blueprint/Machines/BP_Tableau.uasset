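; BP_Tableau is an interactable board machine that displays a hint to the player through a WBP_Hint widget.
; Interract extends the parent logic: while the controller is interacting, it passes Hint to the widget, builds the hints and hides the fusion and slot elements.
; FindHint scans BP_Generate's diagnosis symptoms against the player's found items for ones ready to fuse, but is unfinished and never sets Hint.
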(event EventBeginPlay
  (|CallParentFunction))

(event Collision|EventActorBeginOverlap
  (params (OtherActor :type Actor%20Object%20Reference))
  (|CallParentFunction OtherActor) ; This node is disabled and will not be called.\nDrag off pins to build functionality.
)

(event EventTick
  (params (DeltaSeconds :type Float%20%28single-precision%29))
  (|CallParentFunction DeltaSeconds) ; This node is disabled and will not be called.\nDrag off pins to build functionality.
)

(fn ConstructionScript
  (|CallParentFunction))

(fn Interract
  (|CallParentFunction)
  (if (Variables|/Game/FirstPerson/Blueprints/BP_FirstPersonPlayerController.BP_FirstPersonPlayerController_C|Getis_interacting (CallFunction|GetController))
    (bind _aswbp_hint (Utilities|Casting|CastToWBP_Hint (UserInterface|GetUserWidgetObject (Variables|Default|GetWidget))))
    (Default|SetHint _aswbp_hint (Variables|Default|Gethint))
    (Default|CreateAllHint _aswbp_hint)
    (Default|SetFusionHidden _aswbp_hint)
    (Default|SetSlotHidden _aswbp_hint)))

(fn FindHint
  (bind _returnvalue (Actor|GetActorOfClass "/Game/Blueprint/BP_Generate.BP_Generate_C"))
  (LocalVariables|Setsymptome false)
  (for _array_element (Variables|/Game/Blueprint/Primary_Data_Asset/BP_PDA_Diagnostique.BP_PDA_Diagnostique_C|Getlist_symptome (Variables|/Game/Blueprint/BP_Generate.BP_Generate_C|Getdiagnostique_to_do _returnvalue))
    (if (not (Utilities|Array|ContainsItem (Variables|/Game/FirstPerson/Blueprints/BP_FirstPersonPlayerController.BP_FirstPersonPlayerController_C|Getitem_find (CallFunction|GetController)) _array_element))
      (LocalVariables|Setnot_fusion true)
      (bind _array_element_2 (Utilities|Array|ForEachLoopwithBreak (Variables|/Game/Blueprint/Primary_Data_Asset/BP_PDA_Symptome.BP_PDA_Symptome_C|Getlist_information _array_element) :!label _label)
        (:LoopBody
          (if (not (Utilities|Array|ContainsItem (Variables|/Game/FirstPerson/Blueprints/BP_FirstPersonPlayerController.BP_FirstPersonPlayerController_C|Getitem_find (CallFunction|GetController)) _array_element_2))
            (LocalVariables|Setnot_fusion false)
            (goto _label Break)))
        (:Completed
          (if (LocalVariables|Getnot_fusion)
            _))))))