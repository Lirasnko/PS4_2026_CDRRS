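; Puzzle machine where switches select a function curve to match the target curve of ItemOut.
; On BeginPlay it spawns switches, a validation button and two BP_Fonction_Line plotters feeding the screens, then starts on a random non-target curve.
; Actualise decodes up to four switch bools into a CurveList index, SetBool does the reverse, and the player screen turns green on a match.
; CreateItem spawns the unfound item whose type and function match the selection.
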(event EventBeginPlay
  (bind _player_fonction (Variables|Default|Getplayer_fonction))
  (|CallParentFunction)
  (CallFunction|SetSwitch)
  (CallFunction|SpawnActor)
  (bind _returnvalue (Rendering|Material|CreateDynamicMaterialInstance (Variables|Default|Getscreen) 0 0 "None" :!class /Script/Engine.PrimitiveComponent))
  (Rendering|Material|SetTextureParameterValue _returnvalue "fonction" (Variables|Default|Gettexture_fonction))
  (Rendering|Material|SetScalarParameterValue _returnvalue "speed" (Variables|/Game/Blueprint/Primary_Data_Asset/BP_PDA_Fonction.BP_PDA_Fonction_C|Getspeed (Variables|/Game/Blueprint/Primary_Data_Asset/BP_PDA_Information.BP_PDA_Information_C|Getfonciton (Variables|Default|Getitem_out))) :!class /Script/Engine.MaterialInstanceDynamic)
  (bind _output_get (Variables|Default|Setall_curve_of_type (Variables|Default|Getcurve_list)))
  (Utilities|Array|RemoveItem _output_get (Variables|/Game/Blueprint/Primary_Data_Asset/BP_PDA_Information.BP_PDA_Information_C|Getfonciton (Variables|Default|Getitem_out)))
  (Variables|Default|Setrandom_index (Math|Random|RandomIntegerinRange 0 (Utilities|Array|Length (Variables|Default|Getall_curve_of_type))))
  (for (_array_element _array_index) (Variables|Default|Getcurve_list)
    (if (== _array_element (Utilities|Array|Get(acopy) (Variables|Default|Getall_curve_of_type) (Variables|Default|Getrandom_index)))
      (CallFunction|SetBool _array_index)
      (CallFunction|Actualise)
      (Variables|/Game/Blueprint/BP_Fonction_Line.BP_Fonction_Line_C|Setcurve _player_fonction (Variables|/Game/Blueprint/Primary_Data_Asset/BP_PDA_Fonction.BP_PDA_Fonction_C|Getcurve (Variables|Default|Getfonction_player)))
      (Default|Create _player_fonction)
      (CallFunction|ActualiseScreen (Variables|/Game/Blueprint/BP_Fonction_Line.BP_Fonction_Line_C|Gettarget_image _player_fonction)))))

(event Collision|EventActorBeginOverlap
  (params (OtherActor :type Actor%20Object%20Reference))
  (|CallParentFunction OtherActor) ; This node is disabled and will not be called.\nDrag off pins to build functionality.
)

(event EventTick
  (params (DeltaSeconds :type Float%20%28single-precision%29))
  (|CallParentFunction DeltaSeconds) ; This node is disabled and will not be called.\nDrag off pins to build functionality.
)

(fn ConstructionScript
  (|CallParentFunction))

(fn CreateItem
  (bind _returnvalue (Transformation|GetActorRotation))
  (bind _asbp_first_person_player_controller (CallFunction|GetController))
  (bind _output (Variables|Default|Getoutput))
  (bind _item_find (Variables|/Game/FirstPerson/Blueprints/BP_FirstPersonPlayerController.BP_FirstPersonPlayerController_C|Getitem_find _asbp_first_person_player_controller))
  (bind _relativerotation (Variables|/Script/Engine.SceneComponent|GetRelativeRotation _output))
  (bind (_roll _pitch _yaw) (Math|Rotator|BreakRotator _relativerotation))
  (bind _outassetdata (Class|AssetRegistry|GetAssetsbyClass (Class|AssetRegistryHelpers|GetAssetRegistry) (Class|KismetSystemLibrary|GetClassTopLevelAssetPath "/Game/Blueprint/Primary_Data_Asset/BP_PDA_Information.BP_PDA_Information_C") false))
  (bind _array_element (Utilities|Array|ForEachLoopwithBreak _outassetdata)
    (:LoopBody
      (bind _asbp_pda_information (Utilities|Casting|CastToBP_PDA_Information (Class|AssetRegistryHelpers|GetAsset _array_element)))
      (if (Utilities|Enum|Equal(Enum) (Variables|/Game/Blueprint/Primary_Data_Asset/BP_PDA_Item.BP_PDA_Item_C|Gettype _asbp_pda_information) (Variables|Default|Gettype))
        (Utilities|IsValid (Variables|/Game/Blueprint/Primary_Data_Asset/BP_PDA_Information.BP_PDA_Information_C|Getfonciton _asbp_pda_information)
          (:Is%20Valid
            (if (== (Variables|/Game/Blueprint/Primary_Data_Asset/BP_PDA_Information.BP_PDA_Information_C|Getfonciton _asbp_pda_information) (Variables|Default|Getfonction_player))
              (if (not (Utilities|Array|ContainsItem _item_find _asbp_pda_information))
                (Utilities|Array|Add _item_find _asbp_pda_information)
                (bind _returnvalue_2 (Game|SpawnActorfromClass "/Game/Blueprint/BP_Item.BP_Item_C" (Math|Transform|MakeTransform (+ (Math|Vector|RotateVector (Variables|/Script/Engine.SceneComponent|GetRelativeLocation _output) _returnvalue) (Transformation|GetActorLocation)) (Math|Rotator|MakeRotator (+ _pitch -9e+01) _yaw (+ _roll (.Yaw (Math|Rotator|BreakRotator _returnvalue)) 9e+01)) "1.000000,1.000000,1.000000") "Undefined" "MultiplyWithRoot" 0 0))
                (Variables|/Game/Blueprint/BP_Item.BP_Item_C|Setitem _returnvalue_2 _asbp_pda_information)
                (Default|SetMesh _returnvalue_2)
                (Variables|Default|Setdo_it false)
                (CallFunction|SetLight)
                (|CallParentFunction)))))))))

(fn SetSwitchPosition
  (bind _switch_position (Variables|Default|Getswitch_position))
  (Utilities|Array|Add _switch_position (Variables|Default|Getswicth_01))
  (Utilities|Array|Add _switch_position (Variables|Default|Getswicth_02))
  (Utilities|Array|Add _switch_position (Variables|Default|Getswicth_03))
  (Utilities|Array|Add _switch_position (Variables|Default|Getswicth_04)))

(fn SetSwitchText
  (bind _switch_text (Variables|Default|Getswitch_text))
  (Utilities|Array|Add _switch_text (Variables|Default|Getswitch_name_01))
  (Utilities|Array|Add _switch_text (Variables|Default|Getswitch_name_02))
  (Utilities|Array|Add _switch_text (Variables|Default|Getswitch_name_03))
  (Utilities|Array|Add _switch_text (Variables|Default|Getswitch_name_04)))

(fn Actualise
  (bind _switch_bool (Variables|Default|Getswitch_bool))
  (bind _switch_bool_2 (Variables|Default|Getswitch_bool))
  (bind _switch_bool_3 (Variables|Default|Getswitch_bool))
  (bind _switch_bool_4 (Variables|Default|Getswitch_bool))
  (bind _switch_bool_5 (Variables|Default|Getswitch_bool))
  (bind _switch_bool_6 (Variables|Default|Getswitch_bool))
  (bind _curve_list (Variables|Default|Getcurve_list))
  (bind _returnvalue (Utilities|Array|Length _switch_bool_6))
  (bind _returnvalue_2 (Utilities|Array|Length _switch_bool_2))
  (bind _returnvalue_3 (Utilities|Array|Length _switch_bool_4))
  (bind _output (Utilities|Array|Get(acopy) _switch_bool 3))
  (bind _output_2 (Utilities|Array|Get(acopy) _switch_bool_5 2))
  (bind _output_3 (Utilities|Array|Get(acopy) _switch_bool_3 1))
  (bind _returnvalue_4 (> _returnvalue 3))
  (bind _returnvalue_5 (> _returnvalue_2 1))
  (bind _returnvalue_6 (> _returnvalue_3 2))
  (if (> (Utilities|Array|Length (Variables|Default|Getswitch_bool)) 0)
    (if (Utilities|Array|Get(acopy) (Variables|Default|Getswitch_bool))
      (if _returnvalue_5
        (if _output_3
          (if _returnvalue_6
            (if _output_2
              (if _returnvalue_4
                (if _output
                  (Variables|Default|Setfonction_player (Utilities|Array|Get(acopy) _curve_list) :!label _label)
                  (else
                    (Variables|Default|Setfonction_player (Utilities|Array|Get(acopy) _curve_list 1) :!label _label_2)))
                (else
                  (goto _label)))
              (elif _returnvalue_4
                (if _output
                  (Variables|Default|Setfonction_player (Utilities|Array|Get(acopy) _curve_list 2) :!label _label_3)
                  (else
                    (Variables|Default|Setfonction_player (Utilities|Array|Get(acopy) _curve_list 3) :!label _label_4)))
                (else
                  (goto _label_2))))
            (else
              (goto _label)))
          (elif _returnvalue_6
            (if _output_2
              (if _returnvalue_4
                (if _output
                  (Variables|Default|Setfonction_player (Utilities|Array|Get(acopy) _curve_list 4) :!label _label_5)
                  (else
                    (Variables|Default|Setfonction_player (Utilities|Array|Get(acopy) _curve_list 5) :!label _label_6)))
                (else
                  (goto _label_3)))
              (elif _returnvalue_4
                (if _output
                  (Variables|Default|Setfonction_player (Utilities|Array|Get(acopy) _curve_list 6) :!label _label_7)
                  (else
                    (Variables|Default|Setfonction_player (Utilities|Array|Get(acopy) _curve_list 7) :!label _label_8)))
                (else
                  (goto _label_4))))
            (else
              (goto _label_2))))
        (else
          (goto _label)))
      (elif _returnvalue_5
        (if _output_3
          (if _returnvalue_6
            (if _output_2
              (if _returnvalue_4
                (if _output
                  (Variables|Default|Setfonction_player (Utilities|Array|Get(acopy) _curve_list 8))
                  (else
                    (Variables|Default|Setfonction_player (Utilities|Array|Get(acopy) _curve_list 9))))
                (else
                  (goto _label_5)))
              (elif _returnvalue_4
                (if _output
                  (Variables|Default|Setfonction_player (Utilities|Array|Get(acopy) _curve_list 10))
                  (else
                    (Variables|Default|Setfonction_player (Utilities|Array|Get(acopy) _curve_list 11))))
                (else
                  (goto _label_6))))
            (else
              (goto _label_3)))
          (elif _returnvalue_6
            (if _output_2
              (if _returnvalue_4
                (if _output
                  (Variables|Default|Setfonction_player (Utilities|Array|Get(acopy) _curve_list 12))
                  (else
                    (Variables|Default|Setfonction_player (Utilities|Array|Get(acopy) _curve_list 13))))
                (else
                  (goto _label_7)))
              (elif _returnvalue_4
                (if _output
                  (Variables|Default|Setfonction_player (Utilities|Array|Get(acopy) _curve_list 14))
                  (else
                    (Variables|Default|Setfonction_player (Utilities|Array|Get(acopy) _curve_list 15))))
                (else
                  (goto _label_8))))
            (else
              (goto _label_4))))
        (else
          (goto _label_2))))))

(fn SetSwitch
  (CallFunction|SetSwitchText)
  (CallFunction|SetSwitchPosition)
  (CallFunction|SetSwitchBool))

(fn SetSwitchBool
  (for _index (range 0 (- (Utilities|Array|Length (Variables|Default|Getswitch_name)) 1))
    (Utilities|Array|Add (Variables|Default|Getswitch_bool) false)))

(fn ActualiseScreen
  (params (curve :type Texture%20Render%20Target%202D%20Object%20Reference))
  (bind _fonction_player (Variables|Default|Getfonction_player))
  (bind _returnvalue (Rendering|Material|CreateDynamicMaterialInstance (Variables|Default|Getscreen_player) 0 0 "None" :!class /Script/Engine.PrimitiveComponent))
  (Rendering|Material|SetTextureParameterValue _returnvalue "fonction" curve)
  (Rendering|Material|SetScalarParameterValue _returnvalue "speed" (Variables|/Game/Blueprint/Primary_Data_Asset/BP_PDA_Fonction.BP_PDA_Fonction_C|Getspeed _fonction_player) :!class /Script/Engine.MaterialInstanceDynamic)
  (if (== _fonction_player (Variables|/Game/Blueprint/Primary_Data_Asset/BP_PDA_Information.BP_PDA_Information_C|Getfonciton (Variables|Default|Getitem_out)))
    (Rendering|Material|SetVectorParameterValue _returnvalue "color" "(R=0.000000,G=1.000000,B=0.000000,A=1.000000)" :!class /Script/Engine.MaterialInstanceDynamic)
    (else
      (Rendering|Material|SetVectorParameterValue _returnvalue "color" "(R=1.000000,G=1.000000,B=0.000000,A=1.000000)" :!class /Script/Engine.MaterialInstanceDynamic))))

(fn SetBool
  (params (index :type Integer))
  (bind _switch_bool (Variables|Default|Getswitch_bool))
  (bind _switch_bool_2 (Variables|Default|Getswitch_bool))
  (bind _switch_bool_3 (Variables|Default|Getswitch_bool))
  (bind _switch_bool_4 (Variables|Default|Getswitch_bool))
  (bind _switch_bool_5 (Variables|Default|Getswitch_bool))
  (bind _switch_bool_6 (Variables|Default|Getswitch_bool))
  (bind _switch_bool_7 (Variables|Default|Getswitch_bool))
  (bind _switch_bool_8 (Variables|Default|Getswitch_bool))
  (bind _switch_bool_9 (Variables|Default|Getswitch_bool))
  (bind _switch_bool_10 (Variables|Default|Getswitch_bool))
  (bind _switch_bool_11 (Variables|Default|Getswitch_bool))
  (bind _switch_bool_12 (Variables|Default|Getswitch_bool))
  (bind _switch_bool_13 (Variables|Default|Getswitch_bool))
  (bind _switch_bool_14 (Variables|Default|Getswitch_bool))
  (bind _switch_bool_15 (Variables|Default|Getswitch_bool))
  (bind _switch_bool_16 (Variables|Default|Getswitch_bool))
  (bind _switch_bool_17 (Variables|Default|Getswitch_bool))
  (bind _switch_bool_18 (Variables|Default|Getswitch_bool))
  (bind _switch_bool_19 (Variables|Default|Getswitch_bool))
  (bind _switch_bool_20 (Variables|Default|Getswitch_bool))
  (bind _switch_bool_21 (Variables|Default|Getswitch_bool))
  (bind _switch_bool_22 (Variables|Default|Getswitch_bool))
  (bind _switch_bool_23 (Variables|Default|Getswitch_bool))
  (bind _switch_bool_24 (Variables|Default|Getswitch_bool))
  (bind _switch_bool_25 (Variables|Default|Getswitch_bool))
  (bind _switch_bool_26 (Variables|Default|Getswitch_bool))
  (bind _switch_bool_27 (Variables|Default|Getswitch_bool))
  (bind _switch_bool_28 (Variables|Default|Getswitch_bool))
  (bind _switch_bool_29 (Variables|Default|Getswitch_bool))
  (bind _switch_bool_30 (Variables|Default|Getswitch_bool))
  (if (> (Utilities|Array|Length (Variables|Default|Getswitch_bool)) 3)
    (switch int index
      (:0
        (Utilities|Array|Insert _switch_bool_26 true 3)
        (Utilities|Array|RemoveIndex _switch_bool_26 4)
        (Utilities|Array|Insert _switch_bool_5 true 2 :!label _label)
        (Utilities|Array|RemoveIndex _switch_bool_5 3)
        (Utilities|Array|Insert _switch_bool_4 true 1 :!label _label_2)
        (Utilities|Array|RemoveIndex _switch_bool_4 2)
        (Utilities|Array|Insert _switch_bool_30 true :!label _label_3)
        (Utilities|Array|RemoveIndex _switch_bool_30 1))
      (:1
        (Utilities|Array|Insert _switch_bool_11 false 3)
        (Utilities|Array|RemoveIndex _switch_bool_11 4)
        (goto _label))
      (:2
        (Utilities|Array|Insert _switch_bool_12 true 3)
        (Utilities|Array|RemoveIndex _switch_bool_12 4)
        (Utilities|Array|Insert _switch_bool_6 false 2 :!label _label_4)
        (Utilities|Array|RemoveIndex _switch_bool_6 3)
        (goto _label_2))
      (:3
        (Utilities|Array|Insert _switch_bool_13 false 3)
        (Utilities|Array|RemoveIndex _switch_bool_13 4)
        (goto _label_4))
      (:4
        (Utilities|Array|Insert _switch_bool_16 true 3)
        (Utilities|Array|RemoveIndex _switch_bool_16 4)
        (Utilities|Array|Insert _switch_bool_27 true 2 :!label _label_5)
        (Utilities|Array|RemoveIndex _switch_bool_27 3)
        (Utilities|Array|Insert _switch_bool_3 false 1 :!label _label_6)
        (Utilities|Array|RemoveIndex _switch_bool_3 2)
        (goto _label_3))
      (:5
        (Utilities|Array|Insert _switch_bool_17 false 3)
        (Utilities|Array|RemoveIndex _switch_bool_17 4)
        (goto _label_5))
      (:6
        (Utilities|Array|Insert _switch_bool_14 true 3)
        (Utilities|Array|RemoveIndex _switch_bool_14 4)
        (Utilities|Array|Insert _switch_bool_28 false 2 :!label _label_7)
        (Utilities|Array|RemoveIndex _switch_bool_28 3)
        (goto _label_6))
      (:7
        (Utilities|Array|Insert _switch_bool_15 false 3)
        (Utilities|Array|RemoveIndex _switch_bool_15 4)
        (goto _label_7))
      (:8
        (Utilities|Array|Insert _switch_bool_24 true 3)
        (Utilities|Array|RemoveIndex _switch_bool_24 4)
        (Utilities|Array|Insert _switch_bool_7 true 2 :!label _label_8)
        (Utilities|Array|RemoveIndex _switch_bool_7 3)
        (Utilities|Array|Insert _switch_bool_2 true 1 :!label _label_9)
        (Utilities|Array|RemoveIndex _switch_bool_2 2)
        (Utilities|Array|Insert _switch_bool_29 false :!label _label_10)
        (Utilities|Array|RemoveIndex _switch_bool_29 1))
      (:9
        (Utilities|Array|Insert _switch_bool_25 false 3)
        (Utilities|Array|RemoveIndex _switch_bool_25 4)
        (goto _label_8))
      (:10
        (Utilities|Array|Insert _switch_bool_22 true 3)
        (Utilities|Array|RemoveIndex _switch_bool_22 4)
        (Utilities|Array|Insert _switch_bool_8 false 2 :!label _label_11)
        (Utilities|Array|RemoveIndex _switch_bool_8 3)
        (goto _label_9))
      (:11
        (Utilities|Array|Insert _switch_bool_23 false 3)
        (Utilities|Array|RemoveIndex _switch_bool_23 4)
        (goto _label_11))
      (:12
        (Utilities|Array|Insert _switch_bool_20 true 3)
        (Utilities|Array|RemoveIndex _switch_bool_20 4)
        (Utilities|Array|Insert _switch_bool_9 true 2 :!label _label_12)
        (Utilities|Array|RemoveIndex _switch_bool_9 3)
        (Utilities|Array|Insert _switch_bool false 1 :!label _label_13)
        (Utilities|Array|RemoveIndex _switch_bool 2)
        (goto _label_10))
      (:13
        (Utilities|Array|Insert _switch_bool_21 false 3)
        (Utilities|Array|RemoveIndex _switch_bool_21 4)
        (goto _label_12))
      (:14
        (Utilities|Array|Insert _switch_bool_18 true 3)
        (Utilities|Array|RemoveIndex _switch_bool_18 4)
        (Utilities|Array|Insert _switch_bool_10 false 2 :!label _label_14)
        (Utilities|Array|RemoveIndex _switch_bool_10 3)
        (goto _label_13))
      (:15
        (Utilities|Array|Insert _switch_bool_19 false 3)
        (Utilities|Array|RemoveIndex _switch_bool_19 4)
        (goto _label_14)))
    (elif (> (Utilities|Array|Length (Variables|Default|Getswitch_bool)) 2)
      (switch int index
        (:0
          (goto _label))
        (:1
          (goto _label_4))
        (:2
          (goto _label_5))
        (:3
          (goto _label_7))
        (:4
          (goto _label_8))
        (:5
          (goto _label_11))
        (:6
          (goto _label_12))
        (:7
          (goto _label_14)))
      (elif (> (Utilities|Array|Length (Variables|Default|Getswitch_bool)) 1)
        (switch int index
          (:0
            (goto _label_2))
          (:1
            (goto _label_6))
          (:2
            (goto _label_9))
          (:3
            (goto _label_13)))
        (elif (> (Utilities|Array|Length (Variables|Default|Getswitch_bool)) 0)
          (switch int index
            (:0
              (goto _label_3))
            (:1
              (goto _label_10))))))))

(fn SpawnActor
  (bind _returnvalue (Transformation|GetActorRotation))
  (bind _returnvalue_2 (Transformation|GetActorRotation))
  (bind _bouton_validation (Variables|Default|Getbouton_validation))
  (bind _relativerotation (Variables|/Script/Engine.SceneComponent|GetRelativeRotation _bouton_validation))
  (bind (_roll _pitch _yaw) (Math|Rotator|BreakRotator _relativerotation))
  (bind _returnvalue_3 (Game|SpawnActorfromClass "/Game/Blueprint/Buttons/BP_Button.BP_Button_C" (Math|Transform|MakeTransform (+ (Math|Vector|RotateVector (Variables|/Script/Engine.SceneComponent|GetRelativeLocation _bouton_validation) _returnvalue_2) (Transformation|GetActorLocation)) (Math|Rotator|MakeRotator _roll _pitch (+ _yaw (.Yaw (Math|Rotator|BreakRotator _returnvalue_2)))) "1.000000,1.000000,1.000000") "Undefined" "MultiplyWithRoot" 0 0))
  (Variables|/Game/Blueprint/Buttons/BP_Button.BP_Button_C|Setmachine_parent _returnvalue_3 self)
  (Variables|Default|Setbutton _returnvalue_3)
  (for (_array_element _array_index) (Variables|Default|Getswitch_name)
    (Rendering|Components|TextRender|SetText (Utilities|Array|Get(acopy) (Variables|Default|Getswitch_text) _array_index) _array_element)
    (bind _returnvalue_4 (Game|SpawnActorfromClass "/Game/Blueprint/Buttons/BP_Switch.BP_Switch_C" (Math|Transform|MakeTransform (+ (Math|Vector|RotateVector (Variables|/Script/Engine.SceneComponent|GetRelativeLocation (Utilities|Array|Get(acopy) (Variables|Default|Getswitch_position) _array_index)) _returnvalue) (Transformation|GetActorLocation)) (Math|Rotator|MakeRotator (.Roll (Math|Rotator|BreakRotator (Variables|/Script/Engine.SceneComponent|GetRelativeRotation (Utilities|Array|Get(acopy) (Variables|Default|Getswitch_position) _array_index)))) (.Pitch (Math|Rotator|BreakRotator (Variables|/Script/Engine.SceneComponent|GetRelativeRotation (Utilities|Array|Get(acopy) (Variables|Default|Getswitch_position) _array_index)))) (+ (.Yaw (Math|Rotator|BreakRotator (Variables|/Script/Engine.SceneComponent|GetRelativeRotation (Utilities|Array|Get(acopy) (Variables|Default|Getswitch_position) _array_index)))) (.Yaw (Math|Rotator|BreakRotator _returnvalue)))) "1.000000,1.000000,1.000000") "Undefined" "MultiplyWithRoot" 0 0))
    (Variables|/Game/Blueprint/Buttons/BP_Switch.BP_Switch_C|Setmachine_parent _returnvalue_4 self)
    (Utilities|Array|Add (Variables|Default|Getswitch_list) _returnvalue_4)
    (Variables|/Game/Blueprint/Buttons/BP_Switch.BP_Switch_C|Setindex _returnvalue_4 _array_index))
  (bind _returnvalue_5 (Game|SpawnActorfromClass "/Game/Blueprint/BP_Fonction_Line.BP_Fonction_Line_C" (Math|Transform|MakeTransform (Variables|Default|Getfonction_pos) "0, 0, 0" "1.000000,1.000000,1.000000") "Undefined" "MultiplyWithRoot" 0 0))
  (Variables|/Game/Blueprint/BP_Fonction_Line.BP_Fonction_Line_C|Setcurve _returnvalue_5 (Variables|/Game/Blueprint/Primary_Data_Asset/BP_PDA_Fonction.BP_PDA_Fonction_C|Getcurve (Variables|/Game/Blueprint/Primary_Data_Asset/BP_PDA_Information.BP_PDA_Information_C|Getfonciton (Variables|Default|Getitem_out))))
  (Variables|/Game/Blueprint/BP_Fonction_Line.BP_Fonction_Line_C|Settarget_image _returnvalue_5 (Variables|Default|Gettexture_fonction))
  (Default|Create _returnvalue_5)
  (Utilities|Array|Add (Variables|Default|Getfonction_print) _returnvalue_5)
  (bind _returnvalue_6 (Game|SpawnActorfromClass "/Game/Blueprint/BP_Fonction_Line.BP_Fonction_Line_C" (Math|Transform|MakeTransform (+ (Variables|Default|Getfonction_pos) "300.000000,0.000000,0.000000") "0, 0, 0" "1.000000,1.000000,1.000000") "Undefined" "MultiplyWithRoot" 0 0))
  (bind _output_get (Variables|Default|Setplayer_fonction _returnvalue_6))
  (Variables|/Game/Blueprint/BP_Fonction_Line.BP_Fonction_Line_C|Settarget_image _output_get (Variables|Default|Gettexture_player))
  (Utilities|Array|Add (Variables|Default|Getfonction_print) _returnvalue_6))

(fn Interract)