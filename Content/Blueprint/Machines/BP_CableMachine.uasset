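; BP_CableMachine is a machine Blueprint that opens a cable widget when the player interacts with it.
; On BeginPlay it creates and stores a WBP_Cable widget, passing its cable count and its own world Y position as the cable depth.
; Interract runs the parent logic, then adds the widget to the player screen if the controller is interacting.
; Construction and item creation only call the parent versions.
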(event EventBeginPlay
  (|CallParentFunction)
  (bind _returnvalue (UserInterface|CreateWidget "/Game/Widget/WBP_Cable.WBP_Cable_C" 0 0 0 (Variables|Default|Getcable_count) (.y (Transformation|GetActorLocation))))
  (Variables|Default|Setwidget _returnvalue))

(event EventInterract
  (|CallParentFunction)
  (if (Variables|/Game/FirstPerson/Blueprints/BP_FirstPersonPlayerController.BP_FirstPersonPlayerController_C|Getis_interacting (CallFunction|GetController))
    (UserInterface|Viewport|AddtoPlayerScreen (Variables|Default|Getwidget))))

(fn ConstructionScript
  (|CallParentFunction))

(fn CreateItem
  (|CallParentFunction))