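; BP_Tuto is a tutorial board that shows help text one step at a time.
; On BeginPlay it caches TextTable's row names and shows the first step.
; Each UpdateText call advances the index and reads DT_BoardHelp into BoardText, or into a temporary text component for a couple of middle steps.
; A separate LightOn function swaps spotlight visibility by component tag, without being called here.
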(event EventBeginPlay
  (bind _outrownames (DataTable|GetDataTableRowNames (Variables|Default|Gettext_table)))
  (Variables|Default|Settext _outrownames)
  (CallFunction|UpdateText))

(fn ConstructionScript)

(fn UpdateText
  (bind _index (Variables|Default|Getindex))
  (bind _temp_text (Variables|Default|GetTemp_text))
  (bind _result (Math|Integer|IncrementInt _index)
    (:%20%20
      (Development|PrintString (Utilities|String|ToString(Integer) _index))
      (bind _returnvalue (Utilities|GetDataTableRow "/Game/DT_BoardHelp.DT_BoardHelp" (Utilities|Array|Get(acopy) (Variables|Default|Gettext) _result))
        (:then
          (if (or (< _index 3) (> _index 4))
            (Rendering|SetVisibility (Variables|Default|GetTemp_text) false false)
            (Rendering|Components|TextRender|SetText (Variables|Default|GetBoard_Text) (Utilities|Text|ToText(String) (Utilities|Struct|BreakS_Help _returnvalue)))
            (if (== (Variables|Default|Getindex) 6)
              _)
            (else
              (Rendering|Components|TextRender|SetText _temp_text (Utilities|Text|ToText(String) (Utilities|Struct|BreakS_Help _returnvalue)))
              (Rendering|SetVisibility _temp_text true false))))
        (:RowNotFound
          (Development|PrintString "row not found"))))))

(fn Lighton
  (params (light_on :type Name) (light_off :type Name))
  (bind _self self)
  (bind _self_2 self)
  (bind _returnvalue (Class|Actor|FindComponentbyTag _self "/Script/Engine.SpotLightComponent" light_off))
  (bind _returnvalue_2 (Class|Actor|FindComponentbyTag _self_2 "/Script/Engine.SpotLightComponent" light_on))
  (Utilities|IsValid _returnvalue
    (:Is%20Valid
      (Rendering|SetVisibility _returnvalue false false)
      (Utilities|IsValid _returnvalue_2
        (:Is%20Valid
          (Rendering|SetVisibility _returnvalue_2 true false))
        (:Is%20Not%20Valid
          (Development|PrintString "on not valid"))))))