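; BP_Mouvement_Menu is a menu Blueprint that plays random one-shot animations on a Puppet.
; Each Tick, while the Animation flag is set, a 1-in-150 roll picks a random entry from PuppetAnimation and plays it without looping, so frequency depends on frame rate.
; The flag is cleared during a fixed two-second Delay, then restored, acting as a cooldown independent of clip length.
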(event EventBeginPlay)

(event Collision|EventActorBeginOverlap
  (params (OtherActor :type Actor%20Object%20Reference)))

(event EventTick
  (params (DeltaSeconds :type Float%20%28single-precision%29))
  (bind _puppet_animation (Variables|Default|Getpuppet_animation))
  (if (Variables|Default|Getanimation)
    (if (== (Math|Random|RandomIntegerinRange 0 149) 0)
      (Variables|Default|Setanimation false)
      (Components|Animation|PlayAnimation (Variables|Default|GetPuppet) (Utilities|Array|Get(acopy) _puppet_animation (Math|Random|RandomIntegerinRange 0 (- (Utilities|Array|Length _puppet_animation) 1))) false)
      (Utilities|FlowControl|Delay 2.0)
      (Variables|Default|Setanimation true))))

(fn ConstructionScript
  (|CallParentFunction))