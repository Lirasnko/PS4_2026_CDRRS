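; Menu actor, named for Fusion, whose static mesh plays a spin animation and can show a selection outline.
; playGame runs a Timeline that yaws the mesh through three turns, then re-enables idle animation unless Glowing is set.
; While idle animation is enabled, Tick randomly replays the spin with a small per-frame chance.
; Outline events apply or clear the overlay material, pausing or resuming those random spins.
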(event Custom|setOutlineOn
  (Rendering|Material|SetOverlayMaterial (Variables|Default|GetStaticMesh) "/Game/Materials/Masters/M_Selection_Outline.M_Selection_Outline" :!class /Script/Engine.MeshComponent)
  (Variables|Default|Setanimation false))

(event Custom|setOutlineOff
  (Rendering|Material|SetOverlayMaterial (Variables|Default|GetStaticMesh) 0 :!class /Script/Engine.MeshComponent)
  (Variables|Default|Setanimation true))

(event Custom|playGame
  (bind _newtrack_0 (Timeline|Timeline PlayFromStart)
    (:Update
      (Transformation|SetWorldRotation (Variables|Default|GetStaticMesh) (Math|Rotator|Lerp(Rotator) "0, 0, 0" (Math|Rotator|MakeRotator 0.0 0.0 1.08e+03) _newtrack_0) false false))
    (:Finished
      (if (not (Variables|Default|GetGlowing))
        (Variables|Default|Setanimation true)))))

(event EventBeginPlay)

(event Collision|EventActorBeginOverlap
  (params (OtherActor :type Actor%20Object%20Reference)))

(event EventTick
  (params (DeltaSeconds :type Float%20%28single-precision%29))
  (if (Variables|Default|Getanimation)
    (if (== (Math|Random|RandomIntegerinRange 0 299) 0)
      (Variables|Default|Setanimation false)
      (bind _newtrack_0 (Timeline|Timeline PlayFromStart)
        (:Update
          (Transformation|SetWorldRotation (Variables|Default|GetStaticMesh) (Math|Rotator|Lerp(Rotator) "0, 0, 0" (Math|Rotator|MakeRotator 0.0 0.0 1.08e+03) _newtrack_0) false false))
        (:Finished
          (if (not (Variables|Default|GetGlowing))
            (Variables|Default|Setanimation true)))))))

(fn ConstructionScript)