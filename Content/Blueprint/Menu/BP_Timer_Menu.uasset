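; BP_Timer_Menu is a menu actor that makes a TextRender flicker between two text values at irregular intervals.
; Each Tick has a one-in-a-hundred random chance to flip the Swap boolean and set the matching text.
; No actual timer or countdown runs, so the flip frequency depends on frame rate.
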(event EventBeginPlay)

(event Collision|EventActorBeginOverlap
  (params (OtherActor :type Actor%20Object%20Reference)))

(event EventTick
  (params (DeltaSeconds :type Float%20%28single-precision%29))
  (if (== (Math|Random|RandomIntegerinRange 0 99) 0)
    (if (Variables|Default|Getswap)
      (Variables|Default|Setswap false)
      (Rendering|Components|TextRender|SetText (Variables|Default|GetTextRender) (Variables|Default|GetValue_0))
      (else
        (Variables|Default|Setswap true)
        (Rendering|Components|TextRender|SetText (Variables|Default|GetTextRender) (Variables|Default|GetValue))))))

(fn ConstructionScript)