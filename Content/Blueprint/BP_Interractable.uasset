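; BP_Interractable is an interactable actor with an empty Interract function, apparently meant as a base for child Blueprints.
; On BeginPlay the SKM flag selects the skeletal or static mesh, enabling its visibility and collision and disabling the other's.
; The box collision's visibility follows the skeletal mesh's.
; SetOutlineON and SetOutlineOFF apply or clear a selection-outline overlay material on the active mesh when Glowing is set.
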(event EventBeginPlay
  (bind _mesh (Variables|Default|Getmesh))
  (bind _skeletal_mesh (Variables|Default|Getskeletal_mesh))
  (bind _mesh_2 (Variables|Default|Getmesh))
  (bind _skeletal_mesh_2 (Variables|Default|Getskeletal_mesh))
  (if (Variables|Default|GetSKM)
    (Rendering|SetVisibility _skeletal_mesh true false)
    (Collision|SetCollisionEnabled _skeletal_mesh "QueryAndPhysics")
    (Rendering|SetVisibility _mesh false false)
    (Collision|SetCollisionEnabled _mesh "NoCollision")
    (else
      (Rendering|SetVisibility _skeletal_mesh_2 false false)
      (Collision|SetCollisionEnabled _skeletal_mesh_2 "NoCollision")
      (Rendering|SetVisibility _mesh_2 true false)
      (Collision|SetCollisionEnabled _mesh_2 "QueryAndPhysics")))
  (Rendering|SetVisibility (Variables|Default|Getbox_collision) (Variables|/Script/Engine.SceneComponent|GetbVisible (Variables|Default|Getskeletal_mesh)) false))

(event Collision|EventActorBeginOverlap
  (params (OtherActor :type Actor%20Object%20Reference)))

(event EventTick
  (params (DeltaSeconds :type Float%20%28single-precision%29)))

(fn ConstructionScript)

(fn Interract)

(fn SetOutlineON
  (if (Variables|Default|Getglowing)
    (if (Variables|Default|GetSKM)
      (Rendering|Material|SetOverlayMaterial (Variables|Default|Getskeletal_mesh) "/Game/Materials/Masters/M_Selection_Outline.M_Selection_Outline" :!class /Script/Engine.MeshComponent)
      (else
        (Rendering|Material|SetOverlayMaterial (Variables|Default|Getmesh) "/Game/Materials/Masters/M_Selection_Outline.M_Selection_Outline" :!class /Script/Engine.MeshComponent)))))

(fn SetOutlineOFF
  (if (Variables|Default|Getglowing)
    (if (Variables|Default|GetSKM)
      (Rendering|Material|SetOverlayMaterial (Variables|Default|Getskeletal_mesh) 0 :!class /Script/Engine.MeshComponent)
      (else
        (Rendering|Material|SetOverlayMaterial (Variables|Default|Getmesh) 0 :!class /Script/Engine.MeshComponent)))))