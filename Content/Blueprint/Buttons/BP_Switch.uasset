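; BP_Switch is an animated toggle switch that flips its indexed boolean on a parent machine and shows a selection outline through an overlay material.
; On a BP_Fonction parent it rewrites SwitchBool, then refreshes the function, player curve and screen.
; On a BP_Mouvement parent it toggles InfoBool, updating LEDs for certain indices.
; Indices beyond InfoBool map to MemberBool, where switches are mutually exclusive and the others animate down.
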(event EventBeginPlay)

(event Collision|EventActorBeginOverlap
  (params (OtherActor :type Actor%20Object%20Reference)))

(event EventTick
  (params (DeltaSeconds :type Float%20%28single-precision%29)))

(fn ConstructionScript)

(fn SwitchState
  (bind _machine_parent (Variables|Default|Getmachine_parent))
  (bind _skeletalmesh (Variables|Default|GetSkeletalMesh))
  (bind _bool_list (LocalVariables|Getbool_list))
  (bind _bool_list_2 (LocalVariables|Getbool_list))
  (bind _bool_list_3 (LocalVariables|Getbool_list))
  (bind _bool_list_4 (LocalVariables|Getbool_list))
  (bind _skeletalmesh_2 (Variables|Default|GetSkeletalMesh))
  (bind _index (Variables|Default|Getindex))
  (bind _bool_list_5 (LocalVariables|Getbool_list))
  (bind _skeletalmesh_3 (Variables|Default|GetSkeletalMesh))
  (Utilities|Array|Clear (LocalVariables|Getbool_list))
  (bind _asbp_fonction (Utilities|Casting|CastToBP_Fonction _machine_parent)
    (:then
      (for (_array_element _array_index) (Variables|/Game/Blueprint/Machines/BP_Fonction.BP_Fonction_C|Getswitch_bool _asbp_fonction)
        (if (== _array_index (Variables|Default|Getindex))
          (if _array_element
            (Utilities|Array|Add _bool_list false)
            (Components|Animation|PlayAnimation _skeletalmesh_2 "/Game/Mesh/Buttons_Elements/Toggle_Switch/Animations/AS_Toggle_Switch_GoDown.AS_Toggle_Switch_GoDown" false)
            (else
              (Utilities|Array|Add _bool_list true)
              (Components|Animation|PlayAnimation _skeletalmesh_2 "/Game/Mesh/Buttons_Elements/Toggle_Switch/Animations/AS_Toggle_Switch_GoUp.AS_Toggle_Switch_GoUp" false)))
          (else
            (Utilities|Array|Add (LocalVariables|Getbool_list) _array_element))))
      (Variables|/Game/Blueprint/Machines/BP_Fonction.BP_Fonction_C|Setswitch_bool _asbp_fonction (LocalVariables|Getbool_list))
      (Default|Actualise _asbp_fonction)
      (Variables|/Game/Blueprint/BP_Fonction_Line.BP_Fonction_Line_C|Setcurve (Variables|/Game/Blueprint/Machines/BP_Fonction.BP_Fonction_C|Getplayer_fonction _asbp_fonction) (Variables|/Game/Blueprint/Primary_Data_Asset/BP_PDA_Fonction.BP_PDA_Fonction_C|Getcurve (Variables|/Game/Blueprint/Machines/BP_Fonction.BP_Fonction_C|Getfonction_player _asbp_fonction)))
      (Default|Create (Variables|/Game/Blueprint/Machines/BP_Fonction.BP_Fonction_C|Getplayer_fonction _asbp_fonction))
      (Default|ActualiseScreen _asbp_fonction (Variables|/Game/Blueprint/BP_Fonction_Line.BP_Fonction_Line_C|Gettarget_image (Variables|/Game/Blueprint/Machines/BP_Fonction.BP_Fonction_C|Getplayer_fonction _asbp_fonction))))
    (:CastFailed
      (bind _asbp_mouvement (Utilities|Casting|CastToBP_Mouvement _machine_parent))
      (LocalVariables|Setnot_member true)
      (for (_array_element_2 _array_index_2) (Variables|/Game/Blueprint/Machines/BP_Mouvement.BP_Mouvement_C|Getinfo_bool _asbp_mouvement)
        (if (== _array_index_2 (Variables|Default|Getindex))
          (if _array_element_2
            (Utilities|Array|Add _bool_list_5 false)
            (Components|Animation|PlayAnimation _skeletalmesh_3 "/Game/Mesh/Buttons_Elements/Toggle_Switch/Animations/AS_Toggle_Switch_GoDown.AS_Toggle_Switch_GoDown" false)
            (else
              (Utilities|Array|Add _bool_list_5 true)
              (Components|Animation|PlayAnimation _skeletalmesh_3 "/Game/Mesh/Buttons_Elements/Toggle_Switch/Animations/AS_Toggle_Switch_GoUp.AS_Toggle_Switch_GoUp" false)))
          (LocalVariables|Setnot_member false)
          (else
            (Utilities|Array|Add (LocalVariables|Getbool_list) _array_element_2))))
      (Variables|/Game/Blueprint/Machines/BP_Mouvement.BP_Mouvement_C|Setinfo_bool _asbp_mouvement _bool_list_4)
      (if (LocalVariables|Getnot_member)
        (Utilities|Array|Clear _bool_list_4)
        (for (_array_element_3 _array_index_3) (Variables|/Game/Blueprint/Machines/BP_Mouvement.BP_Mouvement_C|Getmember_bool _asbp_mouvement)
          (if (== (+ (Utilities|Array|Length (Variables|/Game/Blueprint/Machines/BP_Mouvement.BP_Mouvement_C|Getinfo_bool _asbp_mouvement)) _array_index_3) (Variables|Default|Getindex))
            (if _array_element_3
              (Utilities|Array|Add _bool_list_2 false)
              (Components|Animation|PlayAnimation _skeletalmesh "/Game/Mesh/Buttons_Elements/Toggle_Switch/Animations/AS_Toggle_Switch_GoDown.AS_Toggle_Switch_GoDown" false)
              (else
                (Utilities|Array|Add _bool_list_2 true)
                (Components|Animation|PlayAnimation _skeletalmesh "/Game/Mesh/Buttons_Elements/Toggle_Switch/Animations/AS_Toggle_Switch_GoUp.AS_Toggle_Switch_GoUp" false)))
            (elif _array_element_3
              (bind _returnvalue (Utilities|Array|Add _bool_list_3 false))
              (Components|Animation|PlayAnimation (Variables|BP_Switch_C|GetSkeletalMesh (Utilities|Array|Get(acopy) (Variables|/Game/Blueprint/Machines/BP_Mouvement.BP_Mouvement_C|Getmember_switch _asbp_mouvement) _returnvalue)) "/Game/Mesh/Buttons_Elements/Toggle_Switch/Animations/AS_Toggle_Switch_GoDown.AS_Toggle_Switch_GoDown" false)
              (else
                (Utilities|Array|Add _bool_list_3 _array_element_3)))))
        (Variables|/Game/Blueprint/Machines/BP_Mouvement.BP_Mouvement_C|Setmember_bool _asbp_mouvement (LocalVariables|Getbool_list))
        (elif (or (== _index 1) (== _index 3))
          (Default|SetLed _asbp_mouvement))))))

(fn SetOutlineON
  (Rendering|Material|SetOverlayMaterial (Variables|Default|GetSkeletalMesh) "/Game/Materials/MI_Selection_Outline_Button.MI_Selection_Outline_Button" :!class /Script/Engine.MeshComponent))

(fn SetOutlineOFF
  (Rendering|Material|SetOverlayMaterial (Variables|Default|GetSkeletalMesh) 0 :!class /Script/Engine.MeshComponent))