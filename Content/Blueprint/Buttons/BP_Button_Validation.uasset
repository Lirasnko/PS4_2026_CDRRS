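; BP_Button_Validation is a button actor that triggers a validation check on the machine it belongs to.
; Validate casts its MachineParent to BP_Validation and calls ValidationCheck, printing a debug string on success or failure of the cast.
; Two functions toggle a selection outline by setting or clearing an overlay material on the skeletal mesh.
; The event graph and construction script contain no logic.
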(event EventBeginPlay)

(event Collision|EventActorBeginOverlap
  (params (OtherActor :type Actor%20Object%20Reference)))

(event EventTick
  (params (DeltaSeconds :type Float%20%28single-precision%29)))

(fn ConstructionScript)

(fn Validate
  (bind _asbp_validation (Utilities|Casting|CastToBP_Validation (Variables|Default|Getmachine_parent))
    (:then
      (Default|ValidationCheck _asbp_validation)
      (Development|PrintString "checking"))
    (:CastFailed
      (Development|PrintString "not  validation"))))

(fn SetOutlineOFF
  (Rendering|Material|SetOverlayMaterial (Variables|Default|GetSkeletalMesh) 0 :!class /Script/Engine.MeshComponent))

(fn SetOutlineON
  (Rendering|Material|SetOverlayMaterial (Variables|Default|GetSkeletalMesh) "/Game/Materials/MI_Selection_Outline_Button.MI_Selection_Outline_Button" :!class /Script/Engine.MeshComponent))