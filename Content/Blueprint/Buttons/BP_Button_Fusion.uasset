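; BP_Button_Fusion is an interactable button that triggers fusion on its parent machine.
; On interact it runs the machine's fusion checks and rotates the machine toward zero by 72 degrees for each item short of five.
; It then waits one second per missing item before calling CreateItem.
; It flags itself as skeletal-mesh based, so the selection outline overlay goes on that mesh while Glowing is set.
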(event Custom|delayOf
  (params (time :type Float%20%28double-precision%29))
  (Development|PrintString "Animation")
  (Utilities|FlowControl|Delay time)
  (Default|CreateItem (Variables|Default|Getmachine_parent)))

(event EventBeginPlay
  (Variables|Default|SetSKM true)
  (|CallParentFunction))

(event Collision|EventActorBeginOverlap
  (params (OtherActor :type Actor%20Object%20Reference)))

(event EventTick
  (params (DeltaSeconds :type Float%20%28single-precision%29)))

(fn ConstructionScript)

(fn Interract
  (bind _machine_parent (Variables|Default|Getmachine_parent))
  (bind _item_fusion (Variables|/Game/Blueprint/Machines/BP_Fusion.BP_Fusion_C|Getitem_fusion _machine_parent))
  (bind _returnvalue (Utilities|Array|Length _item_fusion))
  (bind _returnvalue_2 (- _returnvalue 5))
  (|CallParentFunction)
  (Default|ItemFusiontoInformationCheck _machine_parent)
  (Default|CheckFusion _machine_parent)
  (Default|RotatetoZero _machine_parent (Transformation|GetWorldRotation (Variables|/Game/Blueprint/BP_Interractable.BP_Interractable_C|Getmesh _machine_parent)) (Math|Conversions|ToFloat(Integer) (* _returnvalue_2 -72)))
  (CallFunction|DelayOf (Math|Conversions|ToFloat(Integer) (* _returnvalue_2 -1))))

(fn SetOutlineON
  (if (Variables|Default|Getglowing)
    (if (Variables|Default|GetSKM)
      (Rendering|Material|SetOverlayMaterial (Variables|Default|Getskeletal_mesh) "/Game/Materials/MI_Selection_Outline_Button.MI_Selection_Outline_Button" :!class /Script/Engine.MeshComponent)
      (else
        (Rendering|Material|SetOverlayMaterial (Variables|Character|GetMesh) "/Game/Materials/MI_Selection_Outline_Button.MI_Selection_Outline_Button" :!class /Script/Engine.MeshComponent)))))