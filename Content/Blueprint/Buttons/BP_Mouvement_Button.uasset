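; BP_Mouvement_Button is a movement button actor that plays a pressed animation and reports to its parent when activated.
; Activate either triggers the parent's animation for its Index or, if DoAnimation is off, spawns a particle system at the button.
; It then appends its Index to the parent's Konami array, recording the press sequence.
; Selection highlighting toggles an outline overlay material on the skeletal mesh.
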(event EventBeginPlay)

(event Collision|EventActorBeginOverlap
  (params (OtherActor :type Actor%20Object%20Reference)))

(event EventTick
  (params (DeltaSeconds :type Float%20%28single-precision%29)))

(fn ConstructionScript)

(fn Activate
  (bind _parent (Variables|Default|Getparent))
  (bind _index (Variables|Default|Getindex))
  (Components|Animation|PlayAnimation (Variables|Default|GetSkeletalMesh) "/Game/Mesh/Buttons_Elements/BT_Rectangle/Animations/AS_BT_Rectangle_Pressed.AS_BT_Rectangle_Pressed" false)
  (if (Variables|/Game/Blueprint/Machines/BP_Mouvement.BP_Mouvement_C|Getdo_animation _parent)
    (Default|Animation _parent _index)
    (else
      (Niagara|SpawnSystematLocation 0 (Transformation|GetActorLocation) (Transformation|GetActorRotation))))
  (Utilities|Array|Add (Variables|/Game/Blueprint/Machines/BP_Mouvement.BP_Mouvement_C|Getkonami (Variables|Default|Getparent)) _index))

(fn SetOutlineON
  (Rendering|Material|SetOverlayMaterial (Variables|Default|GetSkeletalMesh) "/Game/Materials/MI_Selection_Outline_Button.MI_Selection_Outline_Button" :!class /Script/Engine.MeshComponent))

(fn SetOutlineOFF
  (Rendering|Material|SetOverlayMaterial (Variables|Default|GetSkeletalMesh) 0 :!class /Script/Engine.MeshComponent))