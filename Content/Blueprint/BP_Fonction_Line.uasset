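; Actor that draws a float curve as a 3D line, like a function plot, built entirely in the construction script.
; It clears its spline, then samples the curve across its time range, placing points with scaled time on X and value on Z.
; Each pair of neighboring points gets a spline mesh component using SM_Fonction, shaped by the spline's locations and tangents.
; The event graph has no runtime logic.
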(event EventBeginPlay)

(event Collision|EventActorBeginOverlap
  (params (OtherActor :type Actor%20Object%20Reference)))

(event EventTick
  (params (DeltaSeconds :type Float%20%28single-precision%29)))

(fn ConstructionScript
  (bind _curve (Variables|Default|Getcurve))
  (bind (_mintime _maxtime) (Math|Curves|GetTimeRange _curve))
  (Spline|ClearSplinePoints (Variables|Default|GetSpline) true)
  (for _index (range (Math|Float|Truncate (* _mintime 1e+01)) (Math|Float|Truncate (* _maxtime 1e+01)))
    (Spline|AddSplinePointatIndex (Variables|Default|GetSpline) (Math|Vector|MakeVector (* (/ _index (Variables|Default|Getdivider)) 1e+02) 0.0 (* (Math|Curves|GetFloatValue _curve (/ _index (Variables|Default|Getdivider))) 1e+02)) _index "Local" true))
  (for _index_2 (range 0 (- (Spline|GetNumberOfSplinePoints (Variables|Default|GetSpline)) 2))
    (bind _returnvalue (AddComponent|AddSplineMeshComponent false))
    (Components|StaticMesh|SetStaticMesh _returnvalue "/Game/Mesh/SM_Fonction.SM_Fonction")
    (SplineMesh|SetStartandEnd _returnvalue (.Location (Spline|GetLocationandTangentatSplinePoint (Variables|Default|GetSpline) _index_2 "Local")) (.Tangent (Spline|GetLocationandTangentatSplinePoint (Variables|Default|GetSpline) _index_2 "Local")) (.Location (Spline|GetLocationandTangentatSplinePoint (Variables|Default|GetSpline) (+ _index_2 1) "Local")) (.Tangent (Spline|GetLocationandTangentatSplinePoint (Variables|Default|GetSpline) (+ _index_2 1) "Local")) true :!class /Script/Engine.SplineMeshComponent)))