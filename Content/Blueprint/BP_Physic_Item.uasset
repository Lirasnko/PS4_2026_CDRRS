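; BP_Physic_Item is a child item Blueprint that can become a physics object and puffs on impact.
; SetPhysics turns on physics simulation for both its Mesh and SkeletalMesh components.
; Mesh hits spawn the NS_Poof Niagara effect at the mesh location, with a DoPoof flag and delay limiting it to once per second.
; BeginPlay runs the parent logic, then clears the Glowing flag.
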(event OnComponentHit(mesh)
  (params (HitComponent :type Primitive%20Component%20Object%20Reference) (OtherActor :type Actor%20Object%20Reference) (OtherComp :type Primitive%20Component%20Object%20Reference) (NormalImpulse :type Vector :default "0, 0, 0") (Hit :type Hit%20Result%20Structure%20%28by%20ref%29))
  (if (Variables|Default|Getdo_poof)
    (Variables|Default|Setdo_poof false)
    (Niagara|SpawnSystematLocation "/Game/VFX/NS_Poof.NS_Poof" (Transformation|GetWorldLocation (Variables|Character|GetMesh)))
    (Utilities|FlowControl|Delay 1.0)
    (Variables|Default|Setdo_poof true)))

(event EventBeginPlay
  (|CallParentFunction)
  (Variables|Default|Setglowing false))

(event Collision|EventActorBeginOverlap
  (params (OtherActor :type Actor%20Object%20Reference))
  (|CallParentFunction OtherActor) ; This node is disabled and will not be called.\nDrag off pins to build functionality.
)

(event EventTick
  (params (DeltaSeconds :type Float%20%28single-precision%29))
  (|CallParentFunction DeltaSeconds) ; This node is disabled and will not be called.\nDrag off pins to build functionality.
)

(fn ConstructionScript
  (|CallParentFunction))

(fn SetPhysics
  (Physics|SetSimulatePhysics (Variables|Character|GetMesh) true)
  (Physics|SetSimulatePhysics (Variables|Default|Getskeletal_mesh) true))