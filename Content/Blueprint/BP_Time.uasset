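; BP_Time runs the match countdown and triggers the defeat screen when time runs out.
; A looping one-second timer decrements Time, formats it as zero-padded MM:SS and pushes it to the text render of every BP_Timer actor.
; At zero it removes all widgets, blends the view to the BP_MenuCamera with ID 5, then after a short delay shows WBP_Defeat and clears the timer.
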(event Custom|timer
  (bind _output_get (Variables|Default|Settime (- (Variables|Default|Gettime) 1)))
  (if (> (Math|Integer|%(Integer) _output_get 60) 9)
    (if (> (/ (- _output_get (Math|Integer|%(Integer) _output_get 60)) 60) 9)
      (Variables|Default|Settime_text (|GenerictoText (Utilities|String|Append (Utilities|String|ToString(Integer) (/ (- _output_get (Math|Integer|%(Integer) _output_get 60)) 60)) ":" (Utilities|String|ToString(Integer) (Math|Integer|%(Integer) _output_get 60)))))
      (else
        (Variables|Default|Settime_text (|GenerictoText (Utilities|String|Append "0" (Utilities|String|ToString(Integer) (/ (- _output_get (Math|Integer|%(Integer) _output_get 60)) 60)) ":" (Utilities|String|ToString(Integer) (Math|Integer|%(Integer) _output_get 60)))))))
    (elif (> (/ (- _output_get (Math|Integer|%(Integer) _output_get 60)) 60) 9)
      (Variables|Default|Settime_text (|GenerictoText (Utilities|String|Append (Utilities|String|ToString(Integer) (/ (- _output_get (Math|Integer|%(Integer) _output_get 60)) 60)) ":" (Utilities|String|Append "0" (Utilities|String|ToString(Integer) (Math|Integer|%(Integer) _output_get 60))))))
      (else
        (Variables|Default|Settime_text (|GenerictoText (Utilities|String|Append "0" (Utilities|String|ToString(Integer) (/ (- _output_get (Math|Integer|%(Integer) _output_get 60)) 60)) ":" (Utilities|String|Append "0" (Utilities|String|ToString(Integer) (Math|Integer|%(Integer) _output_get 60)))))))))
  (bind _outactors (Actor|GetAllActorsOfClass "/Game/Blueprint/BP_Timer.BP_Timer_C"))
  (for _array_element _outactors
    (bind _asbp_timer (Utilities|Casting|CastToBP_Timer _array_element))
    (Rendering|Components|TextRender|SetText (Variables|/Game/Blueprint/BP_Timer.BP_Timer_C|GetTextRender _asbp_timer) (Variables|Default|Gettime_text)))
  (if (== (Variables|Default|Gettime) 0)
    (Viewport|RemoveAllWidgets)
    (bind _outactors_2 (Actor|GetAllActorsOfClass "/Game/Blueprint/BP_MenuCamera.BP_MenuCamera_C"))
    (for _array_element_2 _outactors_2
      (if (== (Variables|/Game/Blueprint/BP_MenuCamera.BP_MenuCamera_C|GetID _array_element_2) 5)
        (Game|Player|SetViewTargetwithBlend (CallFunction|GetController) _array_element_2 2.0 "VTBlend_Linear" 0.0 false)))
    (Utilities|FlowControl|Delay 2.1)
    (bind _returnvalue (UserInterface|CreateWidget "/Game/Widget/WBP_Defeat.WBP_Defeat_C"))
    (UserInterface|Viewport|AddtoViewport _returnvalue 0)
    (Utilities|Time|ClearandInvalidateTimerbyHandle (stale EventBeginPlay _returnvalue))))

(event EventBeginPlay
  (bind _returnvalue (Utilities|Time|SetTimerbyEvent (delegate Custom|timer) 1.0 true))
  (if (> (Math|Integer|%(Integer) (stale Custom|timer _output_get) 60) 9)
    (if (> (/ (- (stale Custom|timer _output_get) (Math|Integer|%(Integer) (stale Custom|timer _output_get) 60)) 60) 9)
      (Variables|Default|Settime_text (|GenerictoText (Utilities|String|Append (Utilities|String|ToString(Integer) (/ (- (stale Custom|timer _output_get) (Math|Integer|%(Integer) (stale Custom|timer _output_get) 60)) 60)) ":" (Utilities|String|ToString(Integer) (Math|Integer|%(Integer) (stale Custom|timer _output_get) 60)))))
      (else
        (Variables|Default|Settime_text (|GenerictoText (Utilities|String|Append "0" (Utilities|String|ToString(Integer) (/ (- (stale Custom|timer _output_get) (Math|Integer|%(Integer) (stale Custom|timer _output_get) 60)) 60)) ":" (Utilities|String|ToString(Integer) (Math|Integer|%(Integer) (stale Custom|timer _output_get) 60)))))))
    (elif (> (/ (- (stale Custom|timer _output_get) (Math|Integer|%(Integer) (stale Custom|timer _output_get) 60)) 60) 9)
      (Variables|Default|Settime_text (|GenerictoText (Utilities|String|Append (Utilities|String|ToString(Integer) (/ (- (stale Custom|timer _output_get) (Math|Integer|%(Integer) (stale Custom|timer _output_get) 60)) 60)) ":" (Utilities|String|Append "0" (Utilities|String|ToString(Integer) (Math|Integer|%(Integer) (stale Custom|timer _output_get) 60))))))
      (else
        (Variables|Default|Settime_text (|GenerictoText (Utilities|String|Append "0" (Utilities|String|ToString(Integer) (/ (- (stale Custom|timer _output_get) (Math|Integer|%(Integer) (stale Custom|timer _output_get) 60)) 60)) ":" (Utilities|String|Append "0" (Utilities|String|ToString(Integer) (Math|Integer|%(Integer) (stale Custom|timer _output_get) 60)))))))))
  (bind _outactors (Actor|GetAllActorsOfClass "/Game/Blueprint/BP_Timer.BP_Timer_C"))
  (for _array_element _outactors
    (bind _asbp_timer (Utilities|Casting|CastToBP_Timer _array_element))
    (Rendering|Components|TextRender|SetText (Variables|/Game/Blueprint/BP_Timer.BP_Timer_C|GetTextRender _asbp_timer) (Variables|Default|Gettime_text)))
  (if (== (Variables|Default|Gettime) 0)
    (Viewport|RemoveAllWidgets)
    (bind _outactors_2 (Actor|GetAllActorsOfClass "/Game/Blueprint/BP_MenuCamera.BP_MenuCamera_C"))
    (for _array_element_2 _outactors_2
      (if (== (Variables|/Game/Blueprint/BP_MenuCamera.BP_MenuCamera_C|GetID _array_element_2) 5)
        (Game|Player|SetViewTargetwithBlend (CallFunction|GetController) _array_element_2 2.0 "VTBlend_Linear" 0.0 false)))
    (Utilities|FlowControl|Delay 2.1)
    (bind _returnvalue_2 (UserInterface|CreateWidget "/Game/Widget/WBP_Defeat.WBP_Defeat_C"))
    (UserInterface|Viewport|AddtoViewport _returnvalue_2 0)
    (Utilities|Time|ClearandInvalidateTimerbyHandle _returnvalue)))

(event Collision|EventActorBeginOverlap
  (params (OtherActor :type Actor%20Object%20Reference)))

(event EventTick
  (params (DeltaSeconds :type Float%20%28single-precision%29)))

(fn ConstructionScript)