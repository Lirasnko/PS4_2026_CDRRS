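; BP_LinksGame is a Blueprint for what appears to be an early prototype of a click-based link game.
; Clicking component C1 adds it to the first empty set among Link1, Link2 and Link3, through a chain of emptiness checks.
; A1's click and cursor-over events only print a "Clicked" debug string.
; A disconnected copy of the set-filling chain never runs, and the construction script is empty.
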(event OnClicked(C1)
  (params (TouchedComponent :type Primitive%20Component%20Object%20Reference) (ButtonPressed :type Key%20Structure :default "None"))
  (bind _link_1 (Variables|Default|GetLink_1))
  (bind _link_2 (Variables|Default|GetLink_2))
  (bind _link_3 (Variables|Default|GetLink_3))
  (if (Utilities|Set|IsEmpty _link_1)
    (Utilities|Set|Add _link_1 TouchedComponent)
    (elif (Utilities|Set|IsEmpty _link_2)
      (Utilities|Set|Add _link_2 TouchedComponent)
      (elif (Utilities|Set|IsEmpty _link_3)
        (Utilities|Set|Add _link_3 TouchedComponent)))))

(event OnClicked(A1)
  (params (TouchedComponent :type Primitive%20Component%20Object%20Reference) (ButtonPressed :type Key%20Structure :default "None"))
  (Development|PrintString "Clicked"))

(event OnBeginCursorOver(A1)
  (params (TouchedComponent :type Primitive%20Component%20Object%20Reference))
  (Development|PrintString "Clicked"))

(event OnEndCursorOver(A1)
  (params (TouchedComponent :type Primitive%20Component%20Object%20Reference))
  (Development|PrintString "Clicked"))

(fn ConstructionScript)